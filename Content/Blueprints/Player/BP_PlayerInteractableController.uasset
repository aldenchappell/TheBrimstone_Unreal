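; Player interaction controller that finds the interactable under the first-person camera and lets the Interact key trigger it.
; While interaction is allowed, Tick line-traces on Visibility for BPI_Interactable actors and caches the BP_InteractableBase hit.
; A successful press sends InteractMessage and starts an anti-spam delay, during which presses play an invalid sound.
; The BPW_Player icon follows this state, using per-interactable icons from DT_Interactables, a cooldown icon or a default.
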(event `InputAction|InteractKey`
  (params (Key :type "Key Structure"))
  (:`Pressed`
    (if (`KismetSystemLibrary.IsValid` (`self.CurrentInteractable`))
      (if (`self.AllowInteraction`)
        (message `/Game/Blueprints/Interfaces/BPI_Interactable.Interact` (`self.CurrentInteractable`))
        (`self.InteractionDelay`)
        (else
          ;[1 1 1] tell the player they arent looking at an interactable.
          (`GameplayStatics.PlaySound2D` "/Game/Sound/GeneralSFX/InvalidInteractionSound.InvalidInteractionSound" 1.0 1.0 0.0 null null)
          (`self.Set Interaction Image Values` (`self.InteractionCooldownIcon`) (`self.DefaultInteractionIconSize`)))))))

(event `self.ReceiveBeginPlay`
  (`self.UpdateInteractionUI` null)
  (bind _player (`self.GetPlayerRef`)
    (:`Out`
      (set `self.MainCamera` (`/Game/Blueprints/Player/BP_PlayerMain.FirstPersonCamera` _player)))))

(event `self.ReceiveTick`
  (params (DeltaSeconds :type "Float (single-precision)"))
  (if (`self.AllowInteraction`)
    (`self.HandleInteractionLineTrace`)))

(event `InteractionDelay`
  (set `self.AllowInteraction` false)
  (`self.UpdateInteractionUI` (`self.CurrentInteractable`))
  (`KismetSystemLibrary.Delay` (`self.InteractSpamDelay`))
  (set `self.AllowInteraction` true)
  (`self.UpdateInteractionUI` (`self.CurrentInteractable`)))

(fn `HandleInteractionLineTrace`
  (locals (TempInteractable :type "/Game/Blueprints/Environment/Interactables/BP_InteractableBase Object Reference"))
  (bind _maincamera (`self.MainCamera`))
  (bind _returnvalue (`SceneComponent.K2_GetComponentLocation` _maincamera))
  (`/Engine/EditorBlueprintResources/StandardMacros.IsValid` _maincamera
    (:`Is Valid`
      (bind _outhit (`KismetSystemLibrary.LineTraceSingle` _returnvalue (+ _returnvalue (* (`KismetMathLibrary.GetForwardVector` (`SceneComponent.K2_GetComponentRotation` _maincamera)) (`self.InteractionDistance`))) "TraceTypeQuery1"))
      (bind (_bblockinghit _binitialoverlap _time _distance _location _impactpoint _normal _impactnormal _physmat _hitactor) (`GameplayStatics.BreakHitResult` _outhit))
      (if (`KismetSystemLibrary.DoesImplementInterface` _hitactor "/Game/Blueprints/Interfaces/BPI_Interactable.BPI_Interactable_C")
        (bind _asbp_interactable_base (cast `/Game/Blueprints/Environment/Interactables/BP_InteractableBase` _hitactor)
          (:`then`
            (`/Engine/EditorBlueprintResources/StandardMacros.IsValid` _asbp_interactable_base
              (:`Is Valid`
                (bind _output_get (set `self.CurrentInteractable` _asbp_interactable_base))
                (`self.UpdateInteractionUI` _output_get))
              (:`Is Not Valid`
                (set `self.CurrentInteractable` null)
                (return))))
          (:`CastFailed`
            (`self.UpdateInteractionUI` (`self.CurrentInteractable`))
            (return)))
        (else
          (`self.Set Interaction Image Values` (`self.DefaultIcon`) (`self.DefaultIconSize`))
          (set `self.CurrentInteractable` null)
          (return))))))

(fn `Is Looking at Interactable Object`
  (params (target :type "Actor Object Reference"))
  (returns (currentInteractable :type Boolean))
  (bind _currentinteractable (`self.CurrentInteractable`))
  (`/Engine/EditorBlueprintResources/StandardMacros.IsValid` _currentinteractable
    (:`Is Valid`
      (return (== _currentinteractable target)))))

(fn `Set Interaction Image Values`
  (params (Texture :type "Texture2D Object Reference") (IconSize :type "Vector2D Structure"))
  (bind _player (`self.GetPlayerRef`)
    (:`Out`
      (bind _asbpw_player (cast `/Game/Blueprints/Player/UI/BPW_Player` (`/Game/Blueprints/Player/BP_PlayerMain.PlayerUI` _player)))
      (bind (_outimage _outsize) (`/Game/Blueprints/Player/UI/BPW_Player.SetImage` _asbpw_player Texture IconSize))
      (set `/Game/Blueprints/Player/UI/BPW_Player.Out Image` _outimage _asbpw_player)
      (set `/Game/Blueprints/Player/UI/BPW_Player.Out Size` _outsize _asbpw_player))))

(fn `UpdateInteractionUI`
  (params (Interactable :type "/Game/Blueprints/Environment/Interactables/BP_InteractableBase Object Reference"))
  (if (`KismetSystemLibrary.IsValid` (`self.InteractionImage`))
    (`/Engine/EditorBlueprintResources/StandardMacros.IsValid` (`self.CurrentInteractable`)
      (:`Is Valid`
        (if (`self.AllowInteraction`)
          (bind _returnvalue (`|GetDataTableRow` "/Game/Blueprints/DataTables/DT_Interactables.DT_Interactables" (`KismetStringLibrary.Conv_StringToName` (`/Game/Blueprints/Environment/Interactables/BP_InteractableBase.InteractableName` Interactable)))
            (:`then`
              (bind (_interacticon _iconsize) (break `/Game/Blueprints/Structs/STR_Interactables` _returnvalue))
              (`self.Set Interaction Image Values` _interacticon (select `bool` (== _iconsize (0.0 0.0)) :`false` _iconsize :`true` (`self.DefaultInteractionIconSize`))))
            (:`RowNotFound`
              (`self.Set Interaction Image Values` (select `bool` (`self.AllowInteraction`) :`false` (`self.DefaultInteractionIcon`) :`true` (`self.DefaultIcon`)) (`self.DefaultIconSize`))))
          (else
            (`self.Set Interaction Image Values` (`self.InteractionCooldownIcon`) (`self.DefaultInteractionIconSize`)))))
      (:`Is Not Valid`
        (return)))
    (elif (`self.AllowInteraction`)
      (`self.Set Interaction Image Values` (`self.DefaultIcon`) (`self.DefaultIconSize`))
      (return)
      (else
        (`self.Set Interaction Image Values` (`self.DefaultInteractionIcon`) (`self.DefaultInteractionIconSize`))
        (return)))))