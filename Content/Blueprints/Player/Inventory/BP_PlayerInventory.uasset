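; Two-slot player inventory that adds, swaps, removes and places held objects into tag-matched targets.
; Slot inputs set the current index, hide or show items and refresh BPW_Player slot images and highlights via BP_PlayerMain.
; Swaps and pickups special-case "Skull" actors through parent actors, cache original scales, and swaps destroy "GhostPlacement" markers.
; State is split between the struct-based NewInventorySlots and an older InventorySlots array still read by UI code.
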(event EventBeginPlay
  (Variables|Default|SetInventorySlots (Utilities|Array|MakeArray 0 0))
  (Variables|Default|SetCurrentInventoryIndex 0)
  (Utilities|FlowControl|Delay 0.2)
  (bind _playerui (Utilities|MGetReferencetoPlayerUIWidget)
    (:Out
      (Appearance|SetBrushfromTexture (Variables|/Game/Blueprints/Player/UI/BPW_Player.BPW_Player_C|GetInventorySlotImage01 _playerui) "/AudioWidgets/AudioKnobSmall/AudioKnobSmall_TextLayer01.AudioKnobSmall_TextLayer01" false)
      (CallFunction|UpdateInventoryUI self))))

(event EventTick
  (params (DeltaSeconds :type Float%20%28single-precision%29)))

(event Input|ActionEvents|InputActionInventorySlot01
  (params (Key :type Key%20Structure))
  (:Pressed
    (Variables|Default|SetCurrentInventoryIndex 0)
    (CallFunction|ShowCurrentIndexItem)
    (CallFunction|UpdateInventoryUI)))

(event Input|ActionEvents|InputActionInventorySlot02
  (params (Key :type Key%20Structure))
  (:Pressed
    (Variables|Default|SetCurrentInventoryIndex 1)
    (CallFunction|ShowCurrentIndexItem)
    (CallFunction|UpdateInventoryUI)))

(fn SwapObjectsinInventory
  (params (NewObject :type BP%20Interactable%20Base%20Object%20Reference))
  (bind _newinventoryslots (Variables|Default|GetNewInventorySlots))
  (bind _currentinventoryindex (Variables|Default|GetCurrentInventoryIndex))
  (bind _originalscales (Variables|Default|GetOriginalScales))
  (bind _originalscales_2 (Variables|Default|GetOriginalScales))
  (bind _output (Utilities|Array|Get(acopy) _newinventoryslots _currentinventoryindex))
  (bind _output_2 (Utilities|Array|Get(acopy) _newinventoryslots _currentinventoryindex))
  (bind _childactors (Actor|GetAllChildActors (.item _output) true))
  (bind _returnvalue (Transformation|GetActorLocation (.item _output)))
  (bind _returnvalue_2 (Actor|GetParentActor (.item _output_2)))
  (bind _mesh (Variables|/Game/Blueprints/Environment/Interactables/BP_InteractableBase.BP_InteractableBase_C|GetMesh (.item _output_2)))
  (Utilities|Array|SetArrayElem _newinventoryslots _currentinventoryindex (Utilities|Struct|MakeSTR_InventorySlot NewObject))
  (Utilities|FlowControl|Sequence
    (:then_0
      (bind _outactiveinventoryitem (Utilities|MGetCurrentHandItem)
        (:Out
          (if (Utilities|IsValid _outactiveinventoryitem)
            ;[1 1 1] Clear parent
            (Transformation|DetachFromActor _outactiveinventoryitem "KeepRelative" "KeepRelative" "KeepRelative")
            ;[1 1 1] Enable the object
            (Rendering|SetActorHiddenInGame _outactiveinventoryitem false)
            ;[1 1 1] If current slot is NOT tagged skull, enable the collider on the item.
            (Collision|SetCollisionEnabled (Variables|/Game/Blueprints/Environment/Interactables/BP_InteractableBase.BP_InteractableBase_C|GetMesh _outactiveinventoryitem) (select (not (Actor|ActorHasTag _outactiveinventoryitem "Skull")) "QueryAndPhysics" "NoCollision"))
            ;[1 1 1] Functionality to place skull in proper position
            ;;[1 0 0] TODO: HANDLE SKULL SHIT
            (if (Utilities|IsValid _outactiveinventoryitem)
              (bind (_array_element _array_index) (Utilities|Array|ForEachLoopwithBreak _childactors :!label _label)
                (:Completed
                  (if (Utilities|Enum|Equal(Enum) (Utilities|GetDisplayName _array_element) "GhostPlacement")
                    (Transformation|SetActorLocationAndRotation _outactiveinventoryitem (Transformation|GetActorLocation (Utilities|Array|Get(acopy) _childactors _array_index)) (Transformation|GetActorRotation (Utilities|Array|Get(acopy) _childactors _array_index)))
                    (Collision|SetActorEnableCollision _outactiveinventoryitem true)
                    (Rendering|SetActorHiddenInGame _outactiveinventoryitem false)
                    (Utilities|IsValid _outactiveinventoryitem
                      (:Is%20Valid
                        ;;[1 0.03021 0] Destroy the ghost position OBJECT
                        (Actor|DestroyActor (Utilities|Array|Get(acopy) _childactors _array_index))
                        (CallFunction|UpdateInventoryUI :!label _label_2)
                        (return))
                      (:Is%20Not%20Valid
                        (return)))
                    (else
                      (Transformation|SetActorLocationAndRotation (.item _output) _returnvalue (Transformation|GetActorRotation (.item _output)))
                      (Rendering|SetActorHiddenInGame _outactiveinventoryitem false)
                      (Development|PrintString (Utilities|String|ToString(Vector) _returnvalue))
                      (goto _label Break)))))
              (else
                (Transformation|SetActorLocationAndRotation _outactiveinventoryitem (Transformation|GetActorLocation (.item _output)) (Transformation|GetActorRotation (.item _output)))
                (for (_array_element_2 _array_index_2) (Actor|GetAllChildActors _outactiveinventoryitem true)
                  (if (Utilities|Enum|Equal(Enum) "GhostPlacement" (Utilities|GetDisplayName _array_element_2))
                    (Utilities|IsValid _array_element_2
                      (:Is%20Valid
                        ;;[1 0.03021 0] Destroy the ghost position OBJECT
                        (Actor|DestroyActor (Utilities|Array|Get(acopy) (Actor|GetAllChildActors _outactiveinventoryitem true) _array_index_2))
                        (goto _label_2))
                      (:Is%20Not%20Valid
                        (return)))
                    (else
                      (return))))))
            (else
              (return))))))
    (:then_1
      (if (Actor|ActorHasTag (.item _output_2) "Skull")
        (Collision|SetCollisionEnabled _mesh "NoCollision")
        (if (Utilities|IsValid _returnvalue_2)
          (Collision|SetActorEnableCollision _returnvalue_2 true)
          (for _array_element_3 (Actor|GetAllChildActors _returnvalue_2 true)
            (Rendering|SetActorHiddenInGame _outactiveinventoryitem false)
            (Transformation|SetActorTransform _returnvalue_2 (Transformation|GetActorTransform (Game|GetPlayerCharacter 0)))
            (if (not (Utilities|Map|Contains _originalscales_2 0))
              (Utilities|Map|Add _originalscales_2 0 (Class|Actor|GetActorRelativeScale3D (.item _output_2)))
              (|SetBy-RefVar _outactiveinventoryitem (.item _output_2))
              (CallFunction|ShowCurrentIndexItem)
              (goto _label_2)))
          (else
            (return)))
        (else
          (Collision|SetCollisionEnabled _mesh "NoCollision")
          (Actor|SetOwner (Components|GetOwner _mesh) (Game|GetPlayerCharacter 0))
          (if (not (Utilities|Map|Contains _originalscales (.item _output_2)))
            (Utilities|Map|Add _originalscales (.item _output_2) (Class|Actor|GetActorRelativeScale3D (.item _output_2)))
            (|SetBy-RefVar _outactiveinventoryitem (.item _output_2))
            (CallFunction|ShowCurrentIndexItem)
            (goto _label_2)))))))

(fn PlaceObjectfromInventory
  (params (Mesh :type BP%20Interactable%20Base%20Object%20Reference))
  (bind _returnvalue (Actor|GetParentActor Mesh))
  (bind _outactiveinventoryitem (Utilities|MGetCurrentHandItem)
    (:Out
      (if (Utilities|IsValid _outactiveinventoryitem)
        (if (== (Utilities|Name|MakeLiteralName (Utilities|Array|Get(acopy) (Variables|/Script/Engine.Actor|GetTags _outactiveinventoryitem))) (Utilities|Name|MakeLiteralName (Utilities|Array|Get(acopy) (Variables|/Script/Engine.Actor|GetTags Mesh))))
          (if (Utilities|IsValid _returnvalue)
            (Actor|SetOwner Mesh _returnvalue)
            (else
              (Actor|SetOwner Mesh 0)))
          (bind _outactiveinventoryitem_2 (Utilities|MGetCurrentHandItem)
            (:Out
              (Transformation|SetActorLocationAndRotation _outactiveinventoryitem_2 (Transformation|GetActorLocation Mesh) (Transformation|GetActorRotation Mesh))
              (Collision|SetCollisionEnabled (Variables|/Game/Blueprints/Environment/Interactables/BP_InteractableBase.BP_InteractableBase_C|GetMesh _outactiveinventoryitem_2) "QueryAndPhysics")
              (Default|OnPlaceObject Mesh)
              (Components|DestroyComponent (Components|GetChildComponent (Variables|/Game/Blueprints/Environment/Interactables/BP_InteractableBase.BP_InteractableBase_C|GetMesh Mesh) 0))
              (Actor|DestroyActor Mesh)
              ;[1 1 1] will this nullify the currently selected inventory item?
              (Actor|SetOwner _outactiveinventoryitem_2 0)
              (CallFunction|UpdateInventoryUI)
              (return))))
        (else
          (return))))))

(fn OLDRemoveObjectinInventory
  (params (Mesh :type BP%20Interactable%20Base%20Object%20Reference))
  (bind _inventoryslots (Variables|Default|GetInventorySlots))
  (bind (_array_element _array_index) (Utilities|Array|ForEachLoopwithBreak (Variables|Default|GetInventorySlots) :!label _label)
    (:LoopBody
      (Utilities|IsValid _array_element
        (:Is%20Valid
          (if (== (Utilities|Array|Get(acopy) (Variables|/Script/Engine.Actor|GetTags Mesh)) (Utilities|Array|Get(acopy) (Variables|/Script/Engine.Actor|GetTags _array_element)))
            (bind _output_get (LocalVariables|Setindex _array_index))
            (Actor|DestroyActor (Utilities|Array|Get(acopy) _inventoryslots _output_get))
            (Utilities|Array|SetArrayElem _inventoryslots (LocalVariables|Getindex) 0)
            (goto _label Break)
            (else
              (return))))
        (:Is%20Not%20Valid
          (return))))))

(fn HandleMeshVisibility
  (params (Enable :type Boolean))
  ;[1 1 1] If the current inventory slot item is active, enable it. else, disable it.
  (if (Utilities|IsValid (stale _outactiveinventoryitem))
    (if Enable
      (Rendering|SetActorHiddenInGame (stale _outactiveinventoryitem) false)
      (else
        (Rendering|SetActorHiddenInGame (stale _outactiveinventoryitem) true)))
    (return)
    (else
      (return))))

(fn ShowCurrentIndexItem
  (CallFunction|HideHandItem)
  (bind _outactiveinventoryitem (Utilities|MGetCurrentHandItem)
    (:Out
      (if (Utilities|IsValid _outactiveinventoryitem)
        (bind _output_get (LocalVariables|Setitem _outactiveinventoryitem))
        (Rendering|SetActorHiddenInGame _output_get false)
        (Transformation|SetActorLocation (LocalVariables|Getitem) "0, 0, 0" false false)
        (if true
          (if (Utilities|Map|Contains (Variables|Default|GetOriginalScales) (LocalVariables|Getitem))
            (Transformation|SetActorRelativeScale3D (LocalVariables|Getitem) (.Value (Utilities|Map|Find (Variables|Default|GetOriginalScales) (LocalVariables|Getitem))))
            (else
              (Utilities|Map|Add (Variables|Default|GetOriginalScales) (LocalVariables|Getitem) (Class|Actor|GetActorRelativeScale3D (LocalVariables|Getitem)))))
          (Collision|SetActorEnableCollision (LocalVariables|Getitem) false)
          (if (Actor|ActorHasTag (LocalVariables|Getitem) "Skull")
            (Rendering|SetActorHiddenInGame (LocalVariables|Getitem) false)
            (CallFunction|UpdateInventoryUI)
            (return)
            (else
              (return))))
        (else
          (return))))))

(fn PlaceObjectinPuzzle
  (params (obj :type BP%20Interactable%20Base%20Object%20Reference))
  (bind _returnvalue (Actor|GetParentActor obj))
  (bind _inventoryslots (Variables|Default|GetInventorySlots))
  (for (_array_element _array_index) (Variables|Default|GetInventorySlots)
    (if (Utilities|IsValid _array_element)
      (if (== (Utilities|Array|Get(acopy) (Variables|/Script/Engine.Actor|GetTags obj) _array_index) (Utilities|Array|Get(acopy) (Variables|/Script/Engine.Actor|GetTags _array_element) _array_index))
        (bind (_array_element_2 _array_index_2) (Utilities|Array|ForEachLoopwithBreak (Variables|Default|GetInventorySlots) :!label _label)
          (:LoopBody
            (if (== _array_element _array_element_2)
              (LocalVariables|Setindex _array_index_2)
              (goto _label Break)
              (else
                (return))))
          (:Completed
            (if (Utilities|IsValid _returnvalue)
              (Actor|SetOwner (Utilities|Array|Get(acopy) (Variables|Default|GetInventorySlots) (LocalVariables|Getindex)) _returnvalue)
              (else
                (Actor|SetOwner (Utilities|Array|Get(acopy) (Variables|Default|GetInventorySlots) (LocalVariables|Getindex)) 0)))
            (Transformation|SetActorLocationAndRotation (Utilities|Array|Get(acopy) (Variables|Default|GetInventorySlots) (LocalVariables|Getindex)) (Transformation|GetActorLocation obj) (Transformation|GetActorRotation obj))
            (Rendering|SetActorHiddenInGame (Utilities|Array|Get(acopy) (Variables|Default|GetInventorySlots) (LocalVariables|Getindex)) true)
            (Default|OnPlaceObject obj)
            (Actor|DestroyActor obj)
            (Components|DestroyComponent (Class|Actor|GetParentComponent (Utilities|Array|Get(acopy) _inventoryslots (LocalVariables|Getindex))))
            ;[1 1 1] Does this nullify the inventory slot[index]?
            (Utilities|Array|SetArrayElem _inventoryslots (LocalVariables|Getindex) 0)
            (CallFunction|UpdateInventoryUI)
            (return)))
        (else
          (return)))
      (else
        (return)))))

(fn HideHandItem
  (for _array_element (Variables|Default|GetNewInventorySlots)
    (Utilities|IsValid 0
      (:Is%20Valid
        (if (== (Utilities|Array|Get(acopy) (Variables|/Script/Engine.Actor|GetTags (.item _array_element))) "Skull")
          (Collision|SetActorEnableCollision (.item _array_element) false)
          (Transformation|SetActorLocation (.item _array_element) (Transformation|GetWorldLocation (Variables|Default|GetSkullOfHandPosition)) false false)
          (Rendering|SetActorHiddenInGame (.item _array_element) true)
          (else
            (Rendering|SetActorHiddenInGame (.item _array_element) true)))
        (CallFunction|UpdateInventoryUI)
        (return))
      (:Is%20Not%20Valid
        (return)))))

(fn UpdateInventoryUI
  (bind _newinventoryslots (Variables|Default|GetNewInventorySlots))
  (if true
    (Utilities|FlowControl|Sequence
      (:then_0
        (bind _output_get (LocalVariables|SetSelectedSlotColor (Math|Color|MakeColor 255 255 255 255)))
        (LocalVariables|SetInactiveSlotColor (Math|Color|MakeColor (.b _output_get) (.g _output_get) (.r _output_get) 125))
        (for _index (range 0 (Utilities|Array|Length (Variables|Default|GetInventorySlots)))
          (if (Utilities|IsValid (Utilities|Array|Get(acopy) (Variables|Default|GetInventorySlots) _index))
            (if (> (Utilities|Array|Length (Actor|GetComponentsByClass (Utilities|Array|Get(acopy) (Variables|Default|GetInventorySlots) _index) "/Game/Blueprints/Player/Inventory/BP_InventoryObject.BP_InventoryObject_C")) 0)
              (bind _playerui (Utilities|MGetReferencetoPlayerUIWidget)
                (:Out
                  (if (!= (.item (Utilities|Array|Get(acopy) _newinventoryslots)) (.item (Utilities|Array|Get(acopy) _newinventoryslots 1)))
                    (bind (_itemimage _imagescale) (Default|GetItemImage (Utilities|Array|Get(acopy) (Actor|GetComponentsByClass (Utilities|Array|Get(acopy) (Variables|Default|GetInventorySlots) _index) "/Game/Blueprints/Player/Inventory/BP_InventoryObject.BP_InventoryObject_C"))))
                    (Appearance|SetBrushfromTexture (Utilities|Select :Index (Variables|Default|GetCurrentInventoryIndex) :Option%200 (Variables|/Game/Blueprints/Player/UI/BPW_Player.BPW_Player_C|GetInventorySlotImage01 _playerui) :Option%201 (Variables|/Game/Blueprints/Player/UI/BPW_Player.BPW_Player_C|GetInventorySlotImage02 _playerui)) _itemimage false)
                    (Class|WidgetBlueprintLibrary|SetBrushResourcetoTexture (Utilities|Struct|MakeSlateBrush "Image" "NoTile" "NoMirror" _imagescale "(Left=0.000000,Top=0.000000,Right=0.000000,Bottom=0.000000)" "(SpecifiedColor=(R=1.000000,G=1.000000,B=1.000000,A=1.000000),ColorUseRule=UseColor_Specified)" "(CornerRadii=(X=0.000000,Y=0.000000,Z=0.000000,W=1.000000),Color=(SpecifiedColor=(R=0.000000,G=0.000000,B=0.000000,A=0.000000),ColorUseRule=UseColor_Specified),Width=0.000000,RoundingType=HalfHeightRadius,bUseBrushTransparency=False)" 0) _itemimage))
                  (bind _playerui_2 (Utilities|MGetReferencetoPlayerUIWidget)
                    (:Out
                      (Appearance|SetColorandOpacity (Variables|/Game/Blueprints/Player/UI/BPW_Player.BPW_Player_C|GetInventorySlotImage01 _playerui_2) (Variables|/Script/UMG.Image|GetColorAndOpacity (Variables|/Game/Blueprints/Player/UI/BPW_Player.BPW_Player_C|GetInventorySlotImage01 _playerui_2)) :!class /Script/UMG.Image)
                      (Appearance|SetColorandOpacity (Variables|/Game/Blueprints/Player/UI/BPW_Player.BPW_Player_C|GetInventorySlotImage02 _playerui_2) (Variables|/Script/UMG.Image|GetColorAndOpacity (Variables|/Game/Blueprints/Player/UI/BPW_Player.BPW_Player_C|GetInventorySlotImage02 _playerui_2)) :!class /Script/UMG.Image)))))
              (else
                (return)))
            (else
              (bind _playerui_3 (Utilities|MGetReferencetoPlayerUIWidget)
                (:Out
                  (Appearance|SetColorandOpacity (Variables|/Game/Blueprints/Player/UI/BPW_Player.BPW_Player_C|GetInventorySlotImage01 _playerui_3) (Variables|/Script/UMG.Image|GetColorAndOpacity (Variables|/Game/Blueprints/Player/UI/BPW_Player.BPW_Player_C|GetInventorySlotImage01 _playerui_3)) :!class /Script/UMG.Image)
                  (Appearance|SetColorandOpacity (Variables|/Game/Blueprints/Player/UI/BPW_Player.BPW_Player_C|GetInventorySlotImage02 _playerui_3) (Variables|/Script/UMG.Image|GetColorAndOpacity (Variables|/Game/Blueprints/Player/UI/BPW_Player.BPW_Player_C|GetInventorySlotImage02 _playerui_3)) :!class /Script/UMG.Image)))))))
      (:then_1
        (switch int (Variables|Default|GetCurrentInventoryIndex)
          (:Default
            (Development|PrintString "Error assigning UI logic. BP_PlayerInventory/UpdateInventoryUI"))
          (:0
            (bind _playerui_4 (Utilities|MGetReferencetoPlayerUIWidget)
              (:Out
                (Default|SetImageColor _playerui_4 (LocalVariables|GetSelectedSlotColor) (Variables|/Game/Blueprints/Player/UI/BPW_Player.BPW_Player_C|GetInventorySlotBorder01 _playerui_4))
                (Appearance|SetColorandOpacity (Variables|/Game/Blueprints/Player/UI/BPW_Player.BPW_Player_C|GetInventorySlotIndexText01 _playerui_4) (Utilities|Struct|MakeSlateColor (Utilities|Struct|MakeLinearColor (.r (.specifiedcolor (Variables|/Script/UMG.TextBlock|GetColorAndOpacity (Variables|/Game/Blueprints/Player/UI/BPW_Player.BPW_Player_C|GetInventorySlotIndexText01 _playerui_4)))) (.g (.specifiedcolor (Variables|/Script/UMG.TextBlock|GetColorAndOpacity (Variables|/Game/Blueprints/Player/UI/BPW_Player.BPW_Player_C|GetInventorySlotIndexText01 _playerui_4)))) (.b (.specifiedcolor (Variables|/Script/UMG.TextBlock|GetColorAndOpacity (Variables|/Game/Blueprints/Player/UI/BPW_Player.BPW_Player_C|GetInventorySlotIndexText01 _playerui_4)))) 1.0) "UseColor_Specified") :!class /Script/UMG.TextBlock)
                (Appearance|SetColorandOpacity (Variables|/Game/Blueprints/Player/UI/BPW_Player.BPW_Player_C|GetInventorySlotBorder02 _playerui_4) (Math|Conversions|ToLinearColor(Color) (LocalVariables|GetInactiveSlotColor)) :!class /Script/UMG.Image)
                (Appearance|SetColorandOpacity (Variables|/Game/Blueprints/Player/UI/BPW_Player.BPW_Player_C|GetInventorySlotIndexText02 _playerui_4) (Utilities|Struct|MakeSlateColor (Utilities|Struct|MakeLinearColor (.r (.specifiedcolor (Variables|/Script/UMG.TextBlock|GetColorAndOpacity (Variables|/Game/Blueprints/Player/UI/BPW_Player.BPW_Player_C|GetInventorySlotIndexText02 _playerui_4)))) (.g (.specifiedcolor (Variables|/Script/UMG.TextBlock|GetColorAndOpacity (Variables|/Game/Blueprints/Player/UI/BPW_Player.BPW_Player_C|GetInventorySlotIndexText02 _playerui_4)))) (.b (.specifiedcolor (Variables|/Script/UMG.TextBlock|GetColorAndOpacity (Variables|/Game/Blueprints/Player/UI/BPW_Player.BPW_Player_C|GetInventorySlotIndexText02 _playerui_4)))) 0.5) "UseColor_Specified") :!class /Script/UMG.TextBlock))))
          (:1
            (bind _playerui_5 (Utilities|MGetReferencetoPlayerUIWidget)
              (:Out
                (Appearance|SetColorandOpacity (Variables|/Game/Blueprints/Player/UI/BPW_Player.BPW_Player_C|GetInventorySlotBorder02 _playerui_5) (Math|Conversions|ToLinearColor(Color) (LocalVariables|GetSelectedSlotColor)) :!class /Script/UMG.Image)
                (Appearance|SetColorandOpacity (Variables|/Game/Blueprints/Player/UI/BPW_Player.BPW_Player_C|GetInventorySlotIndexText02 _playerui_5) (Utilities|Struct|MakeSlateColor (Utilities|Struct|MakeLinearColor (.r (.specifiedcolor (Variables|/Script/UMG.TextBlock|GetColorAndOpacity (Variables|/Game/Blueprints/Player/UI/BPW_Player.BPW_Player_C|GetInventorySlotIndexText02 _playerui_5)))) (.g (.specifiedcolor (Variables|/Script/UMG.TextBlock|GetColorAndOpacity (Variables|/Game/Blueprints/Player/UI/BPW_Player.BPW_Player_C|GetInventorySlotIndexText02 _playerui_5)))) (.b (.specifiedcolor (Variables|/Script/UMG.TextBlock|GetColorAndOpacity (Variables|/Game/Blueprints/Player/UI/BPW_Player.BPW_Player_C|GetInventorySlotIndexText02 _playerui_5)))) 1.0) "UseColor_Specified") :!class /Script/UMG.TextBlock)
                (Appearance|SetColorandOpacity (Variables|/Game/Blueprints/Player/UI/BPW_Player.BPW_Player_C|GetInventorySlotBorder01 _playerui_5) (Math|Conversions|ToLinearColor(Color) (LocalVariables|GetInactiveSlotColor)) :!class /Script/UMG.Image)
                (Appearance|SetColorandOpacity (Variables|/Game/Blueprints/Player/UI/BPW_Player.BPW_Player_C|GetInventorySlotIndexText01 _playerui_5) (Utilities|Struct|MakeSlateColor (Utilities|Struct|MakeLinearColor (.r (.specifiedcolor (Variables|/Script/UMG.TextBlock|GetColorAndOpacity (Variables|/Game/Blueprints/Player/UI/BPW_Player.BPW_Player_C|GetInventorySlotIndexText01 _playerui_5)))) (.g (.specifiedcolor (Variables|/Script/UMG.TextBlock|GetColorAndOpacity (Variables|/Game/Blueprints/Player/UI/BPW_Player.BPW_Player_C|GetInventorySlotIndexText01 _playerui_5)))) (.b (.specifiedcolor (Variables|/Script/UMG.TextBlock|GetColorAndOpacity (Variables|/Game/Blueprints/Player/UI/BPW_Player.BPW_Player_C|GetInventorySlotIndexText01 _playerui_5)))) 0.5) "UseColor_Specified") :!class /Script/UMG.TextBlock)))))))))

(fn SetCurrentHandItem
  (params (InItem :type BP%20Interactable%20Base%20Object%20Reference))
  (Utilities|Array|SetArrayElem (Variables|Default|GetInventorySlots) (Variables|Default|GetCurrentInventoryIndex) InItem))

(fn HasIteminInventory
  (params (ItemName :type String))
  (bind _outactiveinventoryitem (Utilities|MGetCurrentHandItem)
    (:Out
      (Utilities|IsValid _outactiveinventoryitem
        (:Is%20Valid
          (bind _inventorymeshes (Utilities|MGetInventory)
            (:Out
              (return (Utilities|Enum|Equal(Enum) (Variables|/Game/Blueprints/Environment/Interactables/BP_InteractableBase.BP_InteractableBase_C|GetInteractableName (.item (Utilities|Array|Get(acopy) _inventorymeshes (Variables|Default|GetCurrentInventoryIndex)))) ItemName)))))
        (:Is%20Not%20Valid
          (return false))))))

(fn AddItemtoInventory
  (params (Item :type BP%20Interactable%20Base%20Object%20Reference))
  (bind _returnvalue (Actor|GetParentActor Item))
  (bind _mesh (Variables|/Game/Blueprints/Environment/Interactables/BP_InteractableBase.BP_InteractableBase_C|GetMesh Item))
  (bind _originalscales (Variables|Default|GetOriginalScales))
  (bind _originalscales_2 (Variables|Default|GetOriginalScales))
  (bind _hasitem (CallFunction|HasIteminInventory (Variables|/Game/Blueprints/Environment/Interactables/BP_InteractableBase.BP_InteractableBase_C|GetInteractableName Item)))
  (if (not _hasitem)
    (bind (_array_element _array_index) (Utilities|Array|ForEachLoopwithBreak (Variables|Default|GetNewInventorySlots))
      (:LoopBody
        (Utilities|IsValid (Utilities|Struct|BreakSTR_InventorySlot _array_element)
          (:Is%20Valid
            (return))
          (:Is%20Not%20Valid
            (if true
              (Utilities|Array|SetArrayElem (Variables|Default|GetNewInventorySlots) _array_index (Utilities|Struct|MakeSTR_InventorySlot Item))
              (if (Actor|ActorHasTag Item "Skull")
                (Collision|SetCollisionEnabled _mesh "NoCollision")
                (if (Utilities|IsValid _returnvalue)
                  (Collision|SetActorEnableCollision _returnvalue true)
                  (for _array_element_2 (Actor|GetAllChildActors _returnvalue true)
                    (Rendering|SetActorHiddenInGame Item false)
                    (bind _asbp_player_main (Utilities|Casting|CastToBP_PlayerMain (Game|GetPlayerCharacter 0)))
                    (bind _returnvalue_2 (Transformation|SetActorLocationAndRotation _returnvalue (Transformation|GetWorldLocation (Variables|/Game/Blueprints/Player/BP_PlayerMain.BP_PlayerMain_C|GetSlotOneMesh _asbp_player_main)) (Transformation|GetWorldRotation (Variables|/Game/Blueprints/Player/BP_PlayerMain.BP_PlayerMain_C|GetSlotOneMesh _asbp_player_main))))
                    (if (and _returnvalue_2 (not (Utilities|Map|Contains _originalscales_2 Item)))
                      (Utilities|Map|Add _originalscales_2 Item (Class|Actor|GetActorRelativeScale3D Item))
                      (|SetBy-RefVar Item Item)
                      (CallFunction|ShowCurrentIndexItem)
                      (CallFunction|UpdateInventoryUI)
                      (else
                        (return))))
                  (else
                    (return)))
                (else
                  (Collision|SetCollisionEnabled _mesh "NoCollision")
                  (Actor|SetOwner (Components|GetOwner _mesh) (Game|GetPlayerCharacter 0))
                  (if (not (Utilities|Map|Contains _originalscales Item))
                    (Utilities|Map|Add _originalscales Item (Class|Actor|GetActorRelativeScale3D Item))
                    (|SetBy-RefVar Item Item)
                    (CallFunction|ShowCurrentIndexItem)
                    (CallFunction|UpdateInventoryUI))))
              (else
                (return)))))))))

(fn RemoveItemfromInventory
  (params (Item :type BP%20Interactable%20Base%20Object%20Reference))
  (bind _newinventoryslots (Variables|Default|GetNewInventorySlots))
  (bind (_array_element _array_index) (Utilities|Array|ForEachLoopwithBreak _newinventoryslots :!label _label)
    (:LoopBody
      (if (== (Utilities|Struct|BreakSTR_InventorySlot _array_element) Item)
        (Utilities|Array|SetArrayElem _newinventoryslots _array_index (Utilities|Struct|MakeSTR_InventorySlot 0))
        (CallFunction|UpdateInventoryUI)
        (goto _label Break)
        (else
          (return))))))