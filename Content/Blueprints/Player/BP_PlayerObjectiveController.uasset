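; BP_PlayerObjectiveController holds the player's list of objectives and exposes functions to register and retrieve them.
; RegisterObjective adds an objective when ObjectiveExists reports no match by description, though that check returns after comparing only the first entry.
; UpdateTaskList runs on BeginPlay and after each addition, but it is empty, with its TaskController text update left unconnected.
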(event `self.ReceiveBeginPlay`
  (`self.UpdateTaskList`))

(fn `GetAllObjectives`
  (returns (Objectives :type "Array of /Game/Blueprints/Environment/BP_Objective Object Reference"))
  (return (`self.Objectives`)))

(fn `ObjectiveExists`
  (params (Objective :type String))
  (returns (Exists :type Boolean))
  (for _array_element (`self.Objectives`)
    (return (== (`/Game/Blueprints/Environment/BP_Objective.Description` _array_element) Objective))))

(fn `RegisterObjective`
  (params (Objective :type "/Game/Blueprints/Environment/BP_Objective Object Reference"))
  (bind _exists (`self.ObjectiveExists` (`/Game/Blueprints/Environment/BP_Objective.Description` Objective)))
  (if (not _exists)
    (`KismetArrayLibrary.Array_Add` (`self.Objectives`) Objective)
    (`self.UpdateTaskList`)))

(fn `UpdateTaskList`)