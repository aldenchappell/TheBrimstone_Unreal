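; AI controller for the Furcas demon, which starts its behavior tree and blackboard after the summon animation and picks random patrol nodes.
; Perception sets Chase, speed and player data on sighting, with a delayed realization timer otherwise.
; Line of sight feeds a clamped suspicion value meant to switch Roam and Patrol each Tick, overwriting CurrentState.
; GetSuspicionValue's return is unwired, and ApplyCurrentStateBehavior is an empty stub.
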(event `self.ReceiveBeginPlay`
  (bind _returnvalue (`GameplayStatics.GetActorOfClass` "/Game/Blueprints/Demon/BP_Furcas.BP_Furcas_C"))
  (bind _output_get (set `self.BP_Furcas` _returnvalue))
  (`KismetSystemLibrary.Delay` (`AnimationAsset.GetPlayLength` (`/Game/Blueprints/Demon/BP_Furcas.SummonAnimation` _output_get)))
  (`self.RunBehaviorTree` "/Game/Blueprints/Demon/BT_Furcas.BT_Furcas")
  (bind _blackboardcomponent (`self.UseBlackboard` "/Game/Blueprints/Demon/BB_Furcas.BB_Furcas"))
  (bind _output_get_2 (set `self.Blackboard Component` _blackboardcomponent))
  (set `self.IsBlackboardInitialized?` true)
  (`BlackboardComponent.SetValueAsEnum` _output_get_2 (`self.CurrentState`) (enumliteral `/Game/Blueprints/Data/EN_DemonStates` "NewEnumerator0"))
  (`self.InitLocationNodes`)
  (bind _randompatrolnodelocation (`self.GetRandomLocationNode`))
  (`BlackboardComponent.SetValueAsVector` _output_get_2 (`self.NextNodeLocation`) _randompatrolnodelocation))

(event `self.ReceiveTick`
  (params (DeltaSeconds :type "Float (single-precision)"))
  (bind _blackboard_component (`self.Blackboard Component`))
  (if (`self.IsBlackboardInitialized?`)
    (`self.DetermineCurrentState`)
    (`self.ApplyCurrentStateBehavior`)
    (if (== (`BlackboardComponent.GetValueAsBool` _blackboard_component (`self.HasLineOfSight`)) true)
      (`self.SuspicionTriggered` (`BlackboardComponent.GetValueAsVector` _blackboard_component (`self.PlayerLocation`)) 40.0)
      (else
        (`BlackboardComponent.SetValueAsFloat` _blackboard_component (`self.SusValue`) 0.0)))))

(event `self.AIPerception.OnTargetPerceptionUpdated`
  (params (Actor :type "Actor Object Reference") (Stimulus :type "AIStimulus Structure"))
  (bind _blackboard_component (`self.Blackboard Component`))
  ;[0 0.2668 1] Line Of Sight
  (if (`self.IsBlackboardInitialized?`)
    (if (and (`self.ActorHasTag` Actor "Player") (`.bSuccessfullySensed` (break `AIStimulus` Stimulus)))
      (`KismetSystemLibrary.K2_ClearAndInvalidateTimerHandle` (`self.EnemyTimer`))
      (`/Game/Blueprints/Demon/BP_Furcas.UpdateWalkSpeed` (`self.BP_Furcas`) (`self.ChaseSpeed`))
      (if (`self.IsBlackboardInitialized?`)
        (`BlackboardComponent.SetValueAsVector` _blackboard_component (`self.PlayerLocation`) (`self.K2_GetActorLocation` Actor))
        (`BlackboardComponent.SetValueAsEnum` _blackboard_component (`self.CurrentState`) (enumliteral `/Game/Blueprints/Data/EN_DemonStates` "NewEnumerator1"))
        (`BlackboardComponent.SetValueAsObject` _blackboard_component (`self.Player`) Actor))
      (else
        (bind _returnvalue (`KismetSystemLibrary.K2_SetTimerDelegate` (delegate `RealizationBuffer`) (`BlackboardComponent.GetValueAsFloat` (`self.Blackboard Component`) (`self.RealizationValue`))))
        (set `self.EnemyTimer` _returnvalue)))))

(event `RealizationBuffer`
  ;[0 0.2668 1] Line Of Sight
  (if (`self.IsBlackboardInitialized?`)
    (`BlackboardComponent.SetValueAsObject` (`self.Blackboard Component`) (`self.Player`) (stale `self.AIPerception.OnTargetPerceptionUpdated` Actor))))

(fn `ApplyCurrentStateBehavior`)

(fn `CheckForChaseState`
  (returns (OutChasing :type Boolean))
  (if (`self.IsBlackboardInitialized?`)
    (return (== (`BlackboardComponent.GetValueAsEnum` (`self.Blackboard Component`) (`self.CurrentState`)) (`KismetMathLibrary.Conv_ByteToInt` (`self.ChaseState`))))))

(fn `CheckTime`
  (params (Delta :type "Float (double-precision)"))
  (bind _output_get (set `self.CurrentSpawnTimerValue` Delta))
  (if (>= _output_get (`self.TimeBetweenSpawns`))
    (set `self.CurrentSpawnTimerValue` 0.0)))

(fn `DecreaseTimeToSpawn`
  (params (Value :type Integer))
  (bind _blackboard_component (`self.Blackboard Component`))
  (if (`BlackboardComponent.GetValueAsBool` _blackboard_component (`self.IsPreppingToSpawn`))
    (set `self.CurrentSpawnTimerValue` (+ (`self.CurrentSpawnTimerValue`) Value))
    (else
      (`self.SuspicionTriggered` (`BlackboardComponent.GetValueAsVector` _blackboard_component (`self.PlayerLocation`)) (`KismetMathLibrary.Conv_IntToDouble` Value)))))

(fn `DetermineCurrentState`
  (bind _blackboard_component (`self.Blackboard Component`))
  (if (`self.IsBlackboardInitialized?`)
    (`BlackboardComponent.SetValueAsEnum` _blackboard_component (`self.PreviousState`) (`BlackboardComponent.GetValueAsEnum` _blackboard_component (`self.CurrentState`)))
    (bind _suspicionvalue (`self.GetSuspicionValue`))
    (if (> _suspicionvalue 20.0)
      (`BlackboardComponent.SetValueAsEnum` _blackboard_component (`self.CurrentState`) (enumliteral `/Game/Blueprints/Data/EN_DemonStates` "NewEnumerator2"))
      (else
        (bind _suspicionvalue_2 (`self.GetSuspicionValue`))
        (if (and (> _suspicionvalue_2 0.0) (`|EnumEquality` (cast `/Game/Blueprints/Data/EN_DemonStates` (`BlackboardComponent.GetValueAsEnum` _blackboard_component (`self.CurrentState`))) (enumliteral `/Game/Blueprints/Data/EN_DemonStates` "NewEnumerator0")))
          (`BlackboardComponent.SetValueAsEnum` _blackboard_component (`self.CurrentState`) (enumliteral `/Game/Blueprints/Data/EN_DemonStates` "NewEnumerator2"))
          (else
            (`BlackboardComponent.SetValueAsEnum` _blackboard_component (`self.CurrentState`) (enumliteral `/Game/Blueprints/Data/EN_DemonStates` "NewEnumerator0"))))))))

(fn `GetRandomLocationNode`
  (returns (RandomPatrolNodeLocation :type "Vector Structure"))
  (bind _returnvalue (`self.K2_GetActorLocation` (`KismetArrayLibrary.Array_Random` (`self.LocationNodes`))))
  (`BlackboardComponent.SetValueAsVector` (`AIBlueprintHelperLibrary.GetBlackboard` self) (`self.NextNodeLocation`) _returnvalue)
  (return _returnvalue))

(fn `GetSuspicionValue`
  (returns (SuspicionValue :type "Float (double-precision)"))
  (if (`self.IsBlackboardInitialized?`)
    _))

(fn `InitLocationNodes`
  (bind _outactors (`GameplayStatics.GetAllActorsOfClass` "/Game/Blueprints/Demon/BP_FurcasPatrolNode.BP_FurcasPatrolNode_C"))
  (for _array_element _outactors
    (`KismetArrayLibrary.Array_Add` (`self.LocationNodes`) _array_element)))

(fn `OnReachPatrolPoint`
  (`self.AdjustSuspicionValue` -8.0
    (:`Out`
      (return))))

(fn `RaiseSuspicion`
  (params (Value :type Integer))
  (`self.SuspicionTriggered` (`BlackboardComponent.GetValueAsVector` (`self.Blackboard Component`) (`self.PlayerLocation`)) (`KismetMathLibrary.Conv_IntToDouble` Value)))

(fn `ResetPath`)

(fn `ResetSuspicionValue`
  (if (`self.IsBlackboardInitialized?`)
    (`BlackboardComponent.SetValueAsFloat` (`self.Blackboard Component`) (`self.SusValue`) 0.0)
    (return)))

(fn `SetCurrentMovementState`
  (params (State :type "/Game/Blueprints/Data/EN_DemonStates Enum" :default "NewEnumerator0") (SetPosition :type "Vector Structure"))
  (bind _blackboard_component (`self.Blackboard Component`))
  (if (`self.IsBlackboardInitialized?`)
    (if (and (`BlackboardComponent.GetValueAsBool` _blackboard_component (`self.IsPreppingToSpawn`)) (!= (`BlackboardComponent.GetValueAsVector` _blackboard_component (`self.CurrentEndPosition`)) (0.0 0.0 0.0)))
      (switch `/Game/Blueprints/Data/EN_DemonStates` State))))

(fn `SuspicionTriggered`
  (params (Position :type "Vector Structure") (Value :type "Float (double-precision)"))
  (if (`self.IsBlackboardInitialized?`)
    (`BlackboardComponent.SetValueAsVector` (`self.Blackboard Component`) (`self.LastSuspiciousPosition`) Position)
    (`self.AdjustSuspicionValue` Value)))

(fn `UserConstructionScript`)