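; Game instance that holds progression state: collected keys, completed puzzles and levels, and whether the game is finished.
; CheckAndStartNextLevel picks the first uncompleted of three hard-coded floors and loads its puzzle names, or flags all levels completed.
; A level is saved only when that name list is empty, and player death clears completed puzzles.
; On Init it toggles every BPI_ChangableLight actor according to lobby completion; CompleteObjective is an empty stub.
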(event `self.ReceiveInit`
  (`self.HandleLobbyLights`))

(fn `CheckAndStartNextLevel`
  (`|ExecutionSequence`
    (:`then_0`
      (bind _leveliscompleted_ (`self.IsLevelCompleted` "FLOORONE"))
      (if (not _leveliscompleted_)
        (`self.StartLevel` "FLOORONE" (`self.FloorOnePuzzles`))
        (else
          (bind _leveliscompleted__2 (`self.IsLevelCompleted` "FLOORTWO"))
          (if (not _leveliscompleted__2)
            (`self.StartLevel` "FLOORTWO" (`self.FloorTwoPuzzles`))
            (else
              (bind _leveliscompleted__3 (`self.IsLevelCompleted` "FLOORTHREE"))
              (if (not _leveliscompleted__3)
                (`self.StartLevel` "FLOORTHREE" (`self.FloorThreePuzzles`))
                (else
                  (`self.FinishGame`))))))))))

(fn `CollectKey`
  (`/Engine/EditorBlueprintResources/StandardMacros.IncrementInt` (`self.CollectedKeys`)
    (:`  `
      (set `self.HasKey` true))))

(fn `Complete Objective`
  (params (NewParam :type "/Game/Blueprints/Environment/BP_Objective Object Reference")))

(fn `Complete Puzzle in Scene`
  (params (LevelName :type String) (PuzzleName :type String))
  (locals (LevelNameUpper :type String))
  (bind _completedpuzzles (`self.CompletedPuzzles`))
  (bind _output_get (set `local.LevelNameUpper` (`KismetStringLibrary.ToUpper` LevelName)))
  (if (not (`KismetArrayLibrary.Array_Contains` (`self.CompletedLevels`) _output_get))
    (return)
    (elif (not (`KismetArrayLibrary.Array_Contains` _completedpuzzles PuzzleName))
      (return)
      (else
        (`KismetArrayLibrary.Array_Add` _completedpuzzles PuzzleName)))))

(fn `ConvertPuzzlesToNames`
  (params (Puzzles :type "Array of /Game/Blueprints/Environment/Interactables/Puzzles/BP_InteractablePuzzle Object Reference"))
  (returns (PuzzleNames :type "Array of String"))
  (bind _names (`self.names`))
  (for _array_element Puzzles
    (`KismetArrayLibrary.Array_Add` _names (`/Game/Blueprints/Environment/Interactables/Puzzles/BP_InteractablePuzzle.PuzzleName` _array_element))
    (return _names)))

(fn `FinishGame`
  (set `self.AllLevelsCompleted` true))

(fn `GetCollectedKeys`
  (returns (CollectedKeys :type Integer))
  (return (`self.CollectedKeys`)))

(fn `HandleLobbyLights`
  (locals (ChangableLights :type "Array of Actor Object Reference"))
  (bind _outactors (`GameplayStatics.GetAllActorsWithInterface` "/Game/Blueprints/Environment/Interactables/Lights/BPI_ChangableLight.BPI_ChangableLight_C"))
  (bind _output_get (set `local.ChangableLights` _outactors))
  (for _array_element _output_get
    (if (`self.IsLobbyCompleted`)
      (message `/Game/Blueprints/Environment/Interactables/Lights/BPI_ChangableLight.ToggleLight` _array_element true)
      (else
        (message `/Game/Blueprints/Environment/Interactables/Lights/BPI_ChangableLight.ToggleLight` _array_element false)))))

(fn `IsLevelCompleted`
  (params (LevelName :type String))
  (returns (`LevelIsCompleted?` :type Boolean))
  (return (select `bool` (`KismetArrayLibrary.Array_Contains` (`self.CompletedLevels`) LevelName) :`true` true)))

(fn `OnPlayerDeath`
  (`self.ResetPuzzles`))

(fn `ResetPuzzles`
  (bind _completedpuzzles (`self.CompletedPuzzles`))
  (for _array_element _completedpuzzles
    (`KismetArrayLibrary.Array_RemoveItem` _completedpuzzles _array_element)
    (`KismetArrayLibrary.Array_Clear` _completedpuzzles)))

(fn `SaveLevelCompletion`
  (params (LevelName :type String))
  (if (== (`KismetArrayLibrary.Array_Length` (`self.CurrentLevelPuzzleNames`)) 0)
    (`KismetArrayLibrary.Array_Add` (`self.CompletedLevels`) LevelName)))

(fn `SavePuzzleCompletion`
  (params (Puzzle :type "/Game/Blueprints/Environment/Interactables/Puzzles/BP_InteractablePuzzle Object Reference"))
  (bind _puzzlename (`/Game/Blueprints/Environment/Interactables/Puzzles/BP_InteractablePuzzle.PuzzleName` Puzzle))
  (bind _currentlevelpuzzlenames (`self.CurrentLevelPuzzleNames`))
  (for _array_element (`self.CurrentLevelPuzzleNames`)
    (if (not (`KismetStringLibrary.IsEmpty` _array_element))
      (`KismetArrayLibrary.Array_Add` _currentlevelpuzzlenames _puzzlename)
      (if (`KismetArrayLibrary.Array_Contains` _currentlevelpuzzlenames _puzzlename)
        (`KismetArrayLibrary.Array_RemoveItem` _currentlevelpuzzlenames _puzzlename)))))

(fn `SetCollectedKeys`
  (params (Keys :type Integer))
  (set `self.CollectedKeys` Keys))

(fn `StartLevel`
  (params (LevelName :type String) (Puzzles :type "Array of /Game/Blueprints/Environment/Interactables/Puzzles/BP_InteractablePuzzle Object Reference"))
  (set `self.CurrentLevel` LevelName)
  (bind _puzzlenames (`self.ConvertPuzzlesToNames` Puzzles))
  (set `self.CurrentLevelPuzzleNames` _puzzlenames))