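; Elevator that serves as the level transition between the lobby and three floors, opening its timeline-driven sliding doors on BeginPlay.
; SelectLevel gates travel on collected keys and floor completion read from the game instance, saving completion when returning to the lobby.
; A valid choice closes the doors and runs a delay-timed ding, moving sound and player widget creation before loading the level by name.
; A world-space text widget displays the floor.
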(event `self.ReceiveBeginPlay`
  ;[1 1 1] Start
  (`KismetArrayLibrary.Array_Add` (`self.Doors`) (`|GetArrayItem` (`|MakeArray` (`self.LeftDoor`) (`self.RightDoor`))))
  (`self.OpenElevator`)
  (`self.ShowElevatorLevelOnStart`))

(event `OpenElevator`
  (bind (_direction _elevatorfloat) (`Timeline|ElevatorTimeline` :!label _label)
    (:`Update`
      (`SceneComponent.K2_SetRelativeLocation` (`self.LeftDoor`) (`KismetMathLibrary.VLerp` (`SceneComponent.RelativeLocation` (`self.LeftDoor`)) (0.0 90.0 0.0) _elevatorfloat) false false)
      (`SceneComponent.K2_SetRelativeLocation` (`self.RightDoor`) (`KismetMathLibrary.VLerp` (`SceneComponent.RelativeLocation` (`self.RightDoor`)) (0.0 -180.0 0.0) _elevatorfloat) false false)
      (set `self.IsOpened` (not (`self.IsOpened`))))))

(event `CloseElevator`
  (`self.CloseElevatorRoutine`)
  (goto _label :!via `ReverseFromEnd`))

(event `CloseElevatorRoutine`
  (set `self.IsOpened` false)
  ;[1 1 1] Play Elevator Closing Sound
  (`/Game/Blueprints/Environment/BP_EnvironmentalSoundPlayer.PlaySound2D` (`self.ESP`) (`self.ElevatorClosingSound`))
  (`KismetSystemLibrary.Delay` (`SoundBase.TotalSamples` (`self.ElevatorClosingSound`))))

(event `WaitForLevelEndFade`
  (`KismetSystemLibrary.Delay` (- (`self.TimeBeforeLoadingLevel`) 3.5))
  ;[1 1 1] Create a fade out widget and play it
  (`|CreateWidget` "/Game/Blueprints/Player/UI/BPW_Player.BPW_Player_C" (`GameplayStatics.GetPlayerController` 0)))

(event `StartElevatorRoutine`
  (`GameplayStatics.PlaySound2D` (`self.ElevatorDingSound`) 1.0 1.0 0.0 null null)
  (`KismetSystemLibrary.Delay` (* (+ (`SoundBase.TotalSamples` (`self.ElevatorDingSound`)) 0.5) 0.0001))
  (`GameplayStatics.PlaySound2D` (`self.ElevatorMovingSound`) 1.0 1.0 0.0 null null)
  (`self.WaitForLevelEndFade`)
  (`KismetSystemLibrary.Delay` (- (`self.TimeBeforeLoadingLevel`) 1.0))
  (`GameplayStatics.OpenLevel` (`KismetStringLibrary.Conv_StringToName` (`self.SelectedLevelName`))))

(fn `DisableElevatorButtons`
  (for _array_element (`self.ElevatorButtons`)
    (set `/Game/Blueprints/Environment/Interactables/BP_InteractableBase.IsInteractable` false _array_element)
    (return)))

(fn `SelectLevel`
  (params (FloorIndex :type Integer))
  (bind _selectedlevelname (`self.SelectedLevelName`))
  (bind _outcurrentlevelname (`self.GetCurrentLevelName`)
    (:`Out`
      (bind _asbp_game_instance_class (cast `/Game/Blueprints/Data/BP_GameInstanceClass` (`GameplayStatics.GetGameInstance`))
        (:`then`
          (bind _collectedkeys (`/Game/Blueprints/Data/BP_GameInstanceClass.CollectedKeys` _asbp_game_instance_class))
          (if (and (== _outcurrentlevelname "LOBBY") (>= _collectedkeys 1))
            (return)
            (elif (and (<= _collectedkeys 0) (`KismetStringLibrary.NotEqual_StrStr` _outcurrentlevelname "LOBBY"))
              (return)
              (else
                (bind _outcurrentlevelname_2 (`self.GetCurrentLevelName`)
                  (:`Out`
                    (bind _outgameinstance (`/Game/Blueprints/Reusable/BP_RefToGameInstance.GetRefToGameInstance` (`self.BP_RefToGameInstance`)))
                    (`|ExecutionSequence`
                      (:`then_0`
                        ;[1 1 1] Handle Selecting A Level
                        (switch `int` FloorIndex
                          (:`Default`
                            ;;[1 1 1] Play invalid level sound, Fade out "You do not have permission to access this floor."
                            (return))
                          (:`0`
                            (if (== _outcurrentlevelname_2 "LOBBY")
                              (return)
                              (else
                                (`/Game/Blueprints/Data/BP_GameInstanceClass.SaveLevelCompletion` _outgameinstance (`/Game/Blueprints/Data/BP_GameInstanceClass.CurrentLevel` _outgameinstance))
                                (set `self.SelectedLevelName` "LOBBY"))))
                          (:`1`
                            (set `self.SelectedLevelName` "FLOORONE"))
                          (:`2`
                            (bind _leveliscompleted_ (`/Game/Blueprints/Data/BP_GameInstanceClass.IsLevelCompleted` _outgameinstance "FLOORONE"))
                            (if _leveliscompleted_
                              (set `self.SelectedLevelName` "FLOORTWO")
                              (else
                                ;;[1 1 1] Play invalid level sound, Fade out "You must complete FLOOR ONE first."
                                (return))))
                          (:`3`
                            (bind _leveliscompleted__2 (`/Game/Blueprints/Data/BP_GameInstanceClass.IsLevelCompleted` _outgameinstance "FLOORONE"))
                            (bind _leveliscompleted__3 (`/Game/Blueprints/Data/BP_GameInstanceClass.IsLevelCompleted` _outgameinstance "FLOORTWO"))
                            (if (and _leveliscompleted__3 _leveliscompleted__2)
                              (set `self.SelectedLevelName` "FLOORTHREE")
                              (else
                                ;;[1 1 1] Play invalid level sound, Fade out "You must complete FLOOR ONE and FLOOR TWO first."
                                (return)))))
                        (`self.StartElevatorRoutine`)
                        (return))
                      (:`then_1`
                        (bind _outgameinstance_2 (`/Game/Blueprints/Reusable/BP_RefToGameInstance.GetRefToGameInstance` (`self.BP_RefToGameInstance`)))
                        (bind _leveliscompleted__4 (`/Game/Blueprints/Data/BP_GameInstanceClass.IsLevelCompleted` _outgameinstance_2 _selectedlevelname))
                        (if (and _leveliscompleted__4 (`KismetStringLibrary.NotEqual_StrStr` _selectedlevelname "LOBBY"))
                          (return)
                          (else
                            (set `self.LevelHasBeenSelected` true)
                            (`self.SetElevatorFloorText`)
                            (`self.CloseElevator`)
                            ;[1 1 1] Play level end animation (Fade out)
                            (return)))))))))))
        (:`CastFailed`
          (`KismetSystemLibrary.PrintString` "Couldn't get reference to game instance. BP_Elevator/SelectLevel"))))))

(fn `SetElevatorFloorText`
  (bind _selectedlevelname (`self.SelectedLevelName`))
  (if (`KismetStringLibrary.IsEmpty` _selectedlevelname)
    (return)
    (elif (== _selectedlevelname "LOBBY")
      (`self.SetLevelText` "L"
        (:`Out`
          (return)))
      (elif (== _selectedlevelname "FLOORONE")
        (`self.SetLevelText` "1"
          (:`Out`
            (return)))
        (elif (== _selectedlevelname "FLOORTWO")
          (`self.SetLevelText` "2"
            (:`Out`
              (return)))
          (elif (== _selectedlevelname "FLOORTHREE")
            (`self.SetLevelText` "3"
              (:`Out`
                (return)))
            (else
              (`self.SetLevelText` "L"
                (:`Out`
                  (return))))))))))

(fn `ShowElevatorLevelOnStart`
  (bind _outcurrentlevelname (`self.GetCurrentLevelName`)
    (:`Out`
      (if (`KismetStringLibrary.Contains` _outcurrentlevelname "LOBBY")
        (`self.SetLevelText` "L"
          (:`Out`
            _))
        (elif (`KismetStringLibrary.Contains` _outcurrentlevelname "One")
          (`self.SetLevelText` "1"
            (:`Out`
              _))
          (elif (`KismetStringLibrary.Contains` _outcurrentlevelname "TWO")
            (`self.SetLevelText` "2"
              (:`Out`
                _))
            (else
              (`self.SetLevelText` "3"
                (:`Out`
                  _))))))
      (return))))

(fn `UserConstructionScript`)