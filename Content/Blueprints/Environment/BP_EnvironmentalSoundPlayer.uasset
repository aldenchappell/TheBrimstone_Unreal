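; BP_EnvironmentalSoundPlayer plays environmental sounds as 2D or at a given location, throttled by a shared cooldown.
; Play requests are dropped while CanPlay is false; each accepted one starts a one-second timer that restores it, with one extra second if the Audio component is playing.
; Sounds play fire-and-forget rather than through that component, which the 3D path only repositions using the location as a relative offset.
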(event `StartCooldown`
  (set `self.CanPlay` false)
  (`KismetSystemLibrary.K2_SetTimerDelegate` (delegate `EndCooldown`) 1.0))

(event `EndCooldown`
  (if (`AudioComponent.IsPlaying` (`self.Audio`))
    (`KismetSystemLibrary.Delay` 1.0)
    (set `self.CanPlay` true)
    (else
      (set `self.CanPlay` true))))

(event `PlaySound2D`
  (params (Sound :type "SoundWave Object Reference"))
  (if (`self.CanPlay`)
    (`GameplayStatics.PlaySound2D` Sound 1.0 1.0 0.0 null null)
    (`self.StartCooldown`)))

(event `PlaySound3D`
  (params (Sound :type "SoundWave Object Reference") (Location :type "Vector Structure"))
  (if (`self.CanPlay`)
    (`SceneComponent.K2_SetRelativeLocation` (`self.Audio`) Location false false)
    (`GameplayStatics.PlaySoundAtLocation` Sound Location (struct) 1.0 1.0 0.0 null null null null)
    (`self.StartCooldown`)))

(fn `IsAudioPlaying`
  (returns (OutIsPlaying :type Boolean))
  (return (and (`self.CanPlay`) (`AudioComponent.IsPlaying` (`self.Audio`)))))

(fn `UserConstructionScript`)