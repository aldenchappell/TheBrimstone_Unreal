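; Baby block puzzle interactable for floor two, in which the player rotates a mesh.
; Interacting toggles puzzle mode, swapping to the puzzle camera and enabling the cursor.
; Tick interpolates mesh rotation toward move-axis input, but feeds world location as the current rotation; the WASD-flag RotatePuzzle branch is disconnected.
; CompletePuzzle saves completion through the game instance, though nothing here calls it.
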(event `self.ReceiveBeginPlay`
  (`parent.ReceiveBeginPlay`)
  (bind _asbp_player_main (cast `/Game/Blueprints/Player/BP_PlayerMain` (`GameplayStatics.GetPlayerCharacter` 0)))
  (set `self.Player` _asbp_player_main))

(event `self.ReceiveTick`
  (params (DeltaSeconds :type "Float (single-precision)"))
  (`parent.ReceiveTick` DeltaSeconds)
  (if (`self.InPuzzle`)
    (`self.CheckInput` DeltaSeconds)))

(event `/Game/Blueprints/Interfaces/BPI_Puzzle.TogglePuzzleUI`
  (bind _bp_cursormanager (`self.BP_CursorManager`))
  (set `self.InPuzzle` (not (`self.InPuzzle`)))
  (`/Game/Blueprints/Player/BP_PlayerMain.Swap Camera` (`self.Player`) (`self.PuzzleCamera`))
  (if (`self.InPuzzle`)
    (`/Game/Blueprints/Reusable/BP_CursorManager.EnableCursorAndMovement` _bp_cursormanager true)
    (`self.DisableInput` (`GameplayStatics.GetPlayerController` 0))
    (`self.EnableInput` (`GameplayStatics.GetPlayerController` 0))
    (else
      (`/Game/Blueprints/Reusable/BP_CursorManager.EnableCursorAndMovement` _bp_cursormanager false)
      (`self.DisableInput` null))))

(event `/Game/Blueprints/Interfaces/BPI_Interactable.Interact`
  (if (not (`self.InPuzzle`))
    (`self.TogglePuzzleUI`)))

(event `/Game/Blueprints/Interfaces/BPI_Puzzle.CompletePuzzle`
  (bind _outgameinstance (`/Game/Blueprints/Reusable/BP_RefToGameInstance.GetRefToGameInstance` (`self.BP_RefToGameInstance`)))
  (`/Game/Blueprints/Data/BP_GameInstanceClass.SavePuzzleCompletion` _outgameinstance self)
  (`/Game/Blueprints/Data/BP_GameInstanceClass.Complete Puzzle in Scene` _outgameinstance "FLOORTWO" (`self.PuzzleName`)))

(event `CheckInput`
  (params (DeltaTime :type "Float (double-precision)"))
  (bind _mesh (`self.Mesh`))
  (bind (_returnvalue_x _returnvalue_y _returnvalue_z) (`KismetMathLibrary.BreakVector` (`SceneComponent.K2_GetComponentLocation` _mesh)))
  (bind _output_get (set `self.TargetRotation` (`KismetMathLibrary.MakeRotator` 0.0 (`self.GetInputAxisValue`) (`self.GetInputAxisValue`))))
  (`SceneComponent.K2_SetWorldRotation` _mesh (`KismetMathLibrary.RInterpTo` (`KismetMathLibrary.MakeRotator` _returnvalue_x _returnvalue_y _returnvalue_z) _output_get DeltaTime (`self.RotationSpeed`)) false false))

(event `Key|A`
  (params (Key :type "Key Structure"))
  (:`Pressed`
    (set `self.AKeyPressed` true))
  (:`Released`
    (set `self.AKeyPressed` false)))

(event `Key|D`
  (params (Key :type "Key Structure"))
  (:`Pressed`
    (set `self.DKeyPressed` true))
  (:`Released`
    (set `self.DKeyPressed` false)))

(event `Key|W`
  (params (Key :type "Key Structure"))
  (:`Pressed`
    (set `self.WKeyPressed` true))
  (:`Released`
    (set `self.WKeyPressed` false)))

(event `Key|S`
  (params (Key :type "Key Structure"))
  (:`Pressed`
    (set `self.SKeyPressed` true))
  (:`Released`
    (set `self.SKeyPressed` false)))

(fn `RotatePuzzle`
  (params (Axis :type "Vector Structure") (Angle :type "Float (double-precision)") (DeltaTime :type "Float (double-precision)"))
  (locals (NewRotation :type "Vector Structure"))
  (bind _mesh (`self.Mesh`))
  (bind (_returnvalue_location _returnvalue_rotation) (`KismetMathLibrary.BreakTransform` (`SceneComponent.GetRelativeTransform` _mesh)))
  (bind (_relativerotation_roll _relativerotation_pitch _relativerotation_yaw) (`KismetMathLibrary.BreakRotator` (`SceneComponent.RelativeRotation` (`self.Mesh`))))
  (bind _output_get (set `local.NewRotation` (* (+ _relativerotation_roll _relativerotation_pitch _relativerotation_yaw Axis) Angle)))
  (`SceneComponent.K2_AddWorldRotation` _mesh (`KismetMathLibrary.RLerp` _returnvalue_rotation (`KismetMathLibrary.MakeRotator` (.x _output_get) (.y _output_get) (.z _output_get)) (* DeltaTime 0.0)) false false))

(fn `UserConstructionScript`
  (`parent.UserConstructionScript`))