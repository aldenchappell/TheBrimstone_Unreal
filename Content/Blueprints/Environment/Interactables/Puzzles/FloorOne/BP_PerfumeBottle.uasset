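; Perfume bottle interactable, filed with the Floor One puzzles, that the player picks up into their inventory.
; On Interact it calls PickupItem, then uses the player's BPPlayerInventory component to set itself as the hand item, add itself and refresh the UI.
; PickupItem is empty here, with its DestroyActor node left unconnected, so the function does not destroy the actor.
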(event `/Game/Blueprints/Interfaces/BPI_Interactable.Interact`
  (`self.PickupItem`)
  (bind _asbp_player_main (cast `/Game/Blueprints/Player/BP_PlayerMain` (`GameplayStatics.GetPlayerCharacter` 0)))
  (bind _bp_playerinventory (`/Game/Blueprints/Player/BP_PlayerMain.BP_PlayerInventory` _asbp_player_main))
  (`/Game/Blueprints/Player/Inventory/BP_PlayerInventory.SetCurrentHandItem` _bp_playerinventory self)
  (`/Game/Blueprints/Player/Inventory/BP_PlayerInventory.AddItemToInventory` _bp_playerinventory self)
  (`/Game/Blueprints/Player/Inventory/BP_PlayerInventory.UpdateInventoryUI` _bp_playerinventory))

(fn `PickupItem`
  (returns (Interactable :type "/Game/Blueprints/Environment/Interactables/BP_InteractableBase Object Reference")))

(fn `UserConstructionScript`
  (`parent.UserConstructionScript`))