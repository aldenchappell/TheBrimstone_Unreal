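; BP_Powerbox is the interactable fuse box puzzle in the lobby, which starts open if the game instance marks the lobby completed.
; Interacting swaps to the box camera, enables the cursor and swings the door open on a timeline.
; While open, a Tick cursor trace for BPI_Clickable arms the interact key, which clicks the shadow fuse, or the lever if that fuse is invalid.
; Placing the fuse reveals its mesh and makes the lever interactable.
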(event `self.ReceiveBeginPlay`
  (`parent.ReceiveBeginPlay`)
  (bind _asbp_game_instance_class (cast `/Game/Blueprints/Data/BP_GameInstanceClass` (`GameplayStatics.GetGameInstance`)))
  (if (`/Game/Blueprints/Data/BP_GameInstanceClass.IsLobbyCompleted` _asbp_game_instance_class)
    (`self.OpenPowerBox`)))

(event `/Game/Blueprints/Interfaces/BPI_Interactable.Interact`
  (if (`self.Opened`)
    (`PrimitiveComponent.SetCollisionEnabled` (`self.Mesh`) "QueryAndPhysics")
    (else
      (`self.TogglePuzzleUI`)
      (`self.OpenPowerBox`)
      (`/Game/Blueprints/Reusable/BP_CursorManager.EnableCursorAndMovement` (`self.BP_CursorManager`) true))))

(event `OpenPowerBox`
  (bind _door (`self.Door`))
  (set `self.Opened` true)
  (bind (_direction _dooropenfloat) (`Timeline|Timeline` :!label _label)
    (:`Update`
      (`SceneComponent.K2_SetRelativeLocationAndRotation` (`self.Door`) (`KismetMathLibrary.VInterpTo` (`SceneComponent.RelativeLocation` _door) (`self.New Location`) 0.0 _dooropenfloat) (`KismetMathLibrary.RInterpTo` (`SceneComponent.RelativeRotation` _door) (`KismetMathLibrary.MakeRotator` 0.0 0.0 (`self.DoorOpenAngle`)) 0.0 _dooropenfloat) false false))))

(event `ClosePowerBox`
  (set `self.Opened` false)
  (goto _label :!via `ReverseFromEnd`))

(event `self.OnPlaceObject`
  (params (ItemToPlace :type "/Game/Blueprints/Environment/Interactables/BP_InteractableBase Object Reference (by ref)"))
  (`SceneComponent.SetHiddenInGame` (`self.StaticMeshFuse`) false false)
  (set `/Game/Blueprints/Environment/Interactables/BP_InteractableBase.IsInteractable` true (`self.Lever`)))

(event `InputAction|InteractKey`
  (params (Key :type "Key Structure"))
  (bind _lever (`self.Lever`))
  (bind _shadowfuse (`self.ShadowFuse`))
  (:`Pressed`
    (if (and (`self.CanClick`) (`self.Opened`))
      (`/Engine/EditorBlueprintResources/StandardMacros.IsValid` _shadowfuse
        (:`Is Valid`
          (`/Game/Blueprints/ShadowObjects/BP_ShadowObject.OnClickedEvent` _shadowfuse)
          (set `self.CanClick` false))
        (:`Is Not Valid`
          (`/Engine/EditorBlueprintResources/StandardMacros.IsValid` _lever
            (:`Is Valid`
              (`/Game/Blueprints/Environment/Interactables/Puzzles/Lobby/FuseBox/BP_PowerboxLever.OnClickedEvent` _lever)
              (set `self.CanClick` false))))))))

(event `/Game/Blueprints/Interfaces/BPI_Puzzle.TogglePuzzleUI`
  (bind _returnvalue (`GameplayStatics.GetPlayerController` 0))
  (bind _asbp_player_main (cast `/Game/Blueprints/Player/BP_PlayerMain` (`GameplayStatics.GetPlayerCharacter` 0)))
  (`/Game/Blueprints/Player/BP_PlayerMain.Swap Camera` _asbp_player_main (`self.Camera`))
  (if (`self.Opened`)
    (`self.ClosePowerBox`)
    (`/Game/Blueprints/Reusable/BP_CursorManager.EnableCursorAndMovement` (`self.BP_CursorManager`) false)
    (`self.DisableInput` _returnvalue)
    (else
      (`self.EnableInput` _returnvalue))))

(event `self.ReceiveTick`
  (params (DeltaSeconds :type "Float (single-precision)"))
  (bind (_worldlocation _worlddirection) (`PlayerController.DeprojectMousePositionToWorld` (`GameplayStatics.GetPlayerController` 0)))
  (bind _asbp_game_instance_class (cast `/Game/Blueprints/Data/BP_GameInstanceClass` (`GameplayStatics.GetGameInstance`)))
  (cast `/Game/Blueprints/Player/BP_PlayerMain` (`GameplayStatics.GetPlayerCharacter` 0))
  (if (and (`self.Opened`) (not (`/Game/Blueprints/Data/BP_GameInstanceClass.IsLobbyCompleted` _asbp_game_instance_class)))
    (bind _outhit (`KismetSystemLibrary.LineTraceSingle` _worldlocation (+ _worldlocation (* _worlddirection 500.0)) "TraceTypeQuery1" false (`|MakeArray` (`ActorComponent.GetOwner` (`self.Mesh`)) (`ActorComponent.GetOwner` (`self.SpotLight`)))))
    (if (`KismetSystemLibrary.DoesImplementInterface` (`.HitActor` (`GameplayStatics.BreakHitResult` _outhit)) "/Game/Blueprints/Interfaces/BPI_Clickable.BPI_Clickable_C")
      (set `self.CanClick` true))))

(event `/Game/Blueprints/Interfaces/BPI_Puzzle.CompletePuzzle`
  (bind _outgameinstance (`/Game/Blueprints/Reusable/BP_RefToGameInstance.GetRefToGameInstance` (`self.BP_RefToGameInstance`)))
  (`/Game/Blueprints/Data/BP_GameInstanceClass.Complete Puzzle in Scene` _outgameinstance "" ""))

(fn `UserConstructionScript`
  (`parent.UserConstructionScript`))