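; Baby block puzzle interactable for floor two that the player rotates with WASD.
; Interacting swaps to the puzzle camera, enables the cursor and sets InPuzzle, which lets Tick poll key flags.
; A single held key sends an up or forward axis to RotatePuzzle, which lerps actor rotation at a delta-time-scaled speed.
; CompletePuzzle, not called within this Blueprint, saves completion through the game instance.
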(event `self.ReceiveBeginPlay`
  (`parent.ReceiveBeginPlay`)
  (bind _asbp_player_main (cast `/Game/Blueprints/Player/BP_PlayerMain` (`GameplayStatics.GetPlayerCharacter` 0)))
  (set `self.Player` _asbp_player_main))

(event `self.ReceiveTick`
  (params (DeltaSeconds :type "Float (single-precision)"))
  (`parent.ReceiveTick` DeltaSeconds)
  (if (`self.InPuzzle`)
    (`self.CheckInput` DeltaSeconds)))

(event `/Game/Blueprints/Environment/Interactables/Puzzles/BPI_Puzzle.TogglePuzzleUI`
  (bind _bp_cursormanager (`self.BP_CursorManager`))
  (set `self.InPuzzle` (not (`self.InPuzzle`)))
  (`/Game/Blueprints/Player/BP_PlayerMain.Swap Camera` (`self.Player`) (`self.PuzzleCamera`))
  (if (`self.InPuzzle`)
    (`/Game/Blueprints/Reusable/BP_CursorManager.EnableCursorAndMovement` _bp_cursormanager true)
    (`self.DisableInput` (`GameplayStatics.GetPlayerController` 0))
    (else
      (`/Game/Blueprints/Reusable/BP_CursorManager.EnableCursorAndMovement` _bp_cursormanager false))))

(event `/Game/Blueprints/Environment/Interactables/BPI_Interactable.Interact`
  (if (not (`self.InPuzzle`))
    (`self.TogglePuzzleUI`)))

(event `/Game/Blueprints/Environment/Interactables/Puzzles/BPI_Puzzle.CompletePuzzle`
  (bind _outgameinstance (`/Game/Blueprints/Reusable/BP_RefToGameInstance.GetRefToGameInstance` (`self.BP_RefToGameInstance`)))
  (`/Game/Blueprints/Data/BP_GameInstanceClass.SavePuzzleCompletion` _outgameinstance self)
  (`/Game/Blueprints/Data/BP_GameInstanceClass.Complete Puzzle in Scene` _outgameinstance "FLOORTWO" (`self.PuzzleName`)))

(event `CheckInput`
  (params (DeltaTime :type "Float (double-precision)"))
  (if (and (`self.AKeyPressed`) (not (`self.DKeyPressed`)) (not (`self.WKeyPressed`)) (not (`self.SKeyPressed`)))
    (`self.RotatePuzzle` (`KismetMathLibrary.Vector_Up`) -90.0 DeltaTime)
    (elif (and (`self.DKeyPressed`) (not (`self.AKeyPressed`)) (not (`self.WKeyPressed`)) (not (`self.SKeyPressed`)))
      (`self.RotatePuzzle` (`KismetMathLibrary.Vector_Up`) 90.0 DeltaTime)
      (elif (and (`self.WKeyPressed`) (not (`self.AKeyPressed`)) (not (`self.DKeyPressed`)) (not (`self.SKeyPressed`)))
        (`self.RotatePuzzle` (`KismetMathLibrary.Vector_Forward`) 90.0 DeltaTime)
        (elif (and (`self.SKeyPressed`) (not (`self.AKeyPressed`)) (not (`self.DKeyPressed`)) (not (`self.WKeyPressed`)))
          (`self.RotatePuzzle` (`KismetMathLibrary.Vector_Forward`) -90.0 DeltaTime))))))

(event `Key|A`
  (params (Key :type "Key Structure"))
  (:`Pressed`
    (set `self.AKeyPressed` true))
  (:`Released`
    (set `self.AKeyPressed` false)))

(event `Key|D`
  (params (Key :type "Key Structure"))
  (:`Pressed`
    (set `self.DKeyPressed` true))
  (:`Released`
    (set `self.DKeyPressed` false)))

(event `Key|W`
  (params (Key :type "Key Structure"))
  (:`Pressed`
    (set `self.WKeyPressed` true))
  (:`Released`
    (set `self.WKeyPressed` false)))

(event `Key|S`
  (params (Key :type "Key Structure"))
  (:`Pressed`
    (set `self.SKeyPressed` true))
  (:`Released`
    (set `self.SKeyPressed` false)))

(fn `RotatePuzzle`
  (params (Axis :type "Vector Structure") (Angle :type "Float (double-precision)") (DeltaTime :type "Float (double-precision)"))
  (locals (NewRotation :type "Vector Structure"))
  (bind (_returnvalue_location _returnvalue_rotation) (`KismetMathLibrary.BreakTransform` (`self.GetTransform`)))
  (bind _returnvalue (`self.GetTransform`))
  (bind _output_get (set `local.NewRotation` (* (+ (.roll (.rotation _returnvalue)) (.pitch (.rotation _returnvalue)) (.yaw (.rotation _returnvalue)) Axis) Angle)))
  (`self.K2_SetActorTransform` (`KismetMathLibrary.MakeTransform` (0.0 0.0 0.0) (`KismetMathLibrary.RLerp` _returnvalue_rotation (`KismetMathLibrary.Conv_VectorToRotator` _output_get) (* DeltaTime (`self.RotateSpeedMultiplier`))))))

(fn `UserConstructionScript`
  (`parent.UserConstructionScript`))