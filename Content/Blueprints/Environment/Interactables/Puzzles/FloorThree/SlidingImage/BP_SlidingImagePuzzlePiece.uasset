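; Clickable piece of a sliding image puzzle, which acts as an input relay to its owning Puzzle.
; Its click event passes the piece's Index to the Puzzle's OnPuzzlePieceClicked.
; Cursor enter and exit on both the Box and Mesh toggle the Puzzle's CanClick flag, and each prints a debug "Hello" string.
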(event `self.ReceiveBeginPlay`)

(event `/Game/Blueprints/Interfaces/BPI_Clickable.OnClickedEvent`
  (`/Game/Blueprints/Environment/Interactables/Puzzles/FloorThree/SlidingImage/BP_SlidingImagePuzzle.OnPuzzlePieceClicked` (`self.Puzzle`) (`self.Index`)))

(event `self.Box.OnBeginCursorOver`
  (params (TouchedComponent :type "PrimitiveComponent Object Reference"))
  (set `/Game/Blueprints/Environment/Interactables/Puzzles/FloorThree/SlidingImage/BP_SlidingImagePuzzle.CanClick` true (`self.Puzzle`))
  (`KismetSystemLibrary.PrintString` "Hello" :!label _label))

(event `self.Box.OnEndCursorOver`
  (params (TouchedComponent :type "PrimitiveComponent Object Reference"))
  (set `/Game/Blueprints/Environment/Interactables/Puzzles/FloorThree/SlidingImage/BP_SlidingImagePuzzle.CanClick` false (`self.Puzzle`))
  (goto _label))

(event `self.Mesh.OnBeginCursorOver`
  (params (TouchedComponent :type "PrimitiveComponent Object Reference"))
  (set `/Game/Blueprints/Environment/Interactables/Puzzles/FloorThree/SlidingImage/BP_SlidingImagePuzzle.CanClick` true (`self.Puzzle`))
  (`KismetSystemLibrary.PrintString` "Hello" :!label _label_2))

(event `self.Mesh.OnEndCursorOver`
  (params (TouchedComponent :type "PrimitiveComponent Object Reference"))
  (set `/Game/Blueprints/Environment/Interactables/Puzzles/FloorThree/SlidingImage/BP_SlidingImagePuzzle.CanClick` false (`self.Puzzle`))
  (goto _label_2))

(fn `UserConstructionScript`)