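; Polaroid pickup for the floor three puzzles that goes into the player's inventory and counts toward a polaroid tracker stat.
; Interact makes it the current hand item, adds it to the inventory, refreshes the UI and fires its pickup dispatcher.
; The self-bound handler increases the tracker stat, or only caches the player reference if it is invalid.
; A helper sets a photoboard image to full opacity, keeping its tint.
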(event `self.ReceiveBeginPlay`
  (add `self.OnPickupPolaroid` (delegate `OnPickup`)))

(event `OnPickup`
  (bind _playermainref (`self.PlayerMainRef`))
  (bind _bp_polaroidtracker (`/Game/Blueprints/Player/BP_PlayerMain.BP_PolaroidTracker` _playermainref))
  (`/Engine/EditorBlueprintResources/StandardMacros.IsValid` _playermainref
    (:`Is Valid`
      (`/Game/Blueprints/Player/Stats/BP_PlayerLevelStatTracker.IncreaseStat` _bp_polaroidtracker (`/Game/Blueprints/Player/Stats/BP_PlayerLevelStatTracker.StatName` _bp_polaroidtracker) (`/Game/Blueprints/Player/Stats/BP_PlayerLevelStatTracker.StatValue` _bp_polaroidtracker)))
    (:`Is Not Valid`
      (bind _asbp_player_main (cast `/Game/Blueprints/Player/BP_PlayerMain` (`GameplayStatics.GetPlayerCharacter` 0)))
      (set `self.PlayerMainRef` _asbp_player_main))))

(event `/Game/Blueprints/Interfaces/BPI_Interactable.Interact`
  (bind _bp_playerinventory (`/Game/Blueprints/Player/BP_PlayerMain.BP_PlayerInventory` (`self.PlayerMainRef`)))
  (`self.PickupItem`)
  (`/Game/Blueprints/Player/Inventory/BP_PlayerInventory.SetCurrentHandItem` _bp_playerinventory self)
  (`/Game/Blueprints/Player/Inventory/BP_PlayerInventory.AddItemToInventory` _bp_playerinventory self)
  (`/Game/Blueprints/Player/Inventory/BP_PlayerInventory.UpdateInventoryUI` _bp_playerinventory)
  (`self.OnPickupPolaroid`))

(fn `PickupItem`
  (returns (Interactable :type "/Game/Blueprints/Environment/Interactables/BP_InteractableBase Object Reference"))
  (return self))

(fn `SetPhotoboardImageAlpha`
  (params (Image :type "Image Object Reference"))
  (bind (_drawas _tiling _mirroring _imagesize _margin _tintcolor) (break `SlateBrush` (`Image.Brush` Image)))
  (`Image.SetColorAndOpacity` Image (make `LinearColor` (break `LinearColor` (break `SlateColor` _tintcolor)) (`.G` (break `LinearColor` (break `SlateColor` _tintcolor))) (`.B` (break `LinearColor` (break `SlateColor` _tintcolor))) 1.0)))

(fn `UserConstructionScript`
  (`parent.UserConstructionScript`))