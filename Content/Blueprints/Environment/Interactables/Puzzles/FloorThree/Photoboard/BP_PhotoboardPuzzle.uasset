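; Interactable photoboard puzzle that switches to a puzzle camera and lets the player click slot pieces within a move limit.
; A cursor line trace finds the hovered slot, and a move counter resets the puzzle at the limit or triggers a check.
; The check compares slot materials with UI polaroid images; completion saves progress and spawns a key.
; Material randomisation, UI refresh and objective completion are empty stubs here.
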(event `InputAction|InteractKey`
  (params (Key :type "Key Structure"))
  (bind _currenthoveredpuzzlepiece (`self.CurrentHoveredPuzzlePiece`))
  (:`Pressed`
    (if (and (`KismetSystemLibrary.IsValid` _currenthoveredpuzzlepiece) (`self.CanClick`))
      (`/Game/Blueprints/Environment/Interactables/Puzzles/FloorThree/Photoboard/BP_PhotoboardPuzzleSlot.OnClickedEvent` _currenthoveredpuzzlepiece))))

(event `self.ReceiveBeginPlay`
  (`parent.ReceiveBeginPlay`)
  (add `self.OnReachedMaxMoves` (delegate `/Game/Blueprints/Interfaces/BPI_Puzzle.ResetPuzzle`))
  (add `self.OnMoveMade` (delegate `/Game/Blueprints/Interfaces/BPI_Puzzle.MakeMove`))
  (bind _asbpw_bp_photoboard_puzzle_widget_actor (cast `/Game/Blueprints/Environment/Interactables/Puzzles/FloorThree/Photoboard/BPW_BP_PhotoboardPuzzleWidgetActor` (`WidgetComponent.GetWidget` (`self.Widget`))))
  (set `self.PuzzleUI` _asbpw_bp_photoboard_puzzle_widget_actor)
  (bind _asbp_player_main (cast `/Game/Blueprints/Player/BP_PlayerMain` (`GameplayStatics.GetPlayerCharacter` 0)))
  (set `self.Player` _asbp_player_main)
  (`self.ResetPuzzle`)
  (add `self.OnPuzzleCompletion` (delegate `/Game/Blueprints/Interfaces/BPI_Puzzle.CompletePuzzle`)))

(event `/Game/Blueprints/Interfaces/BPI_Puzzle.CompletePuzzle`
  (bind _outgameinstance (`/Game/Blueprints/Reusable/BP_RefToGameInstance.GetRefToGameInstance` (`self.BP_RefToGameInstance`)))
  (`/Game/Blueprints/Data/BP_GameInstanceClass.Complete Puzzle in Scene` _outgameinstance "FLOORTWO" (`self.PuzzleName`))
  (`/Game/Blueprints/Data/BP_GameInstanceClass.SavePuzzleCompletion` _outgameinstance self)
  (`/Game/Blueprints/Data/BP_GameInstanceClass.SpawnKey` _outgameinstance)
  (set `self.Solved` true)
  (`self.CompleteObjective`))

(event `/Game/Blueprints/Interfaces/BPI_Puzzle.ResetPuzzle`
  (set `self.MovesMade` 0)
  (`self.UpdatePuzzleUI`)
  (`self.AssignRandomMaterials`))

(event `/Game/Blueprints/Interfaces/BPI_Puzzle.MakeMove`
  (bind _movesmade (`self.MovesMade`))
  (`/Engine/EditorBlueprintResources/StandardMacros.IncrementInt` _movesmade
    (:`  `
      (if (>= _movesmade (`self.MaxMoves`))
        (`self.ResetPuzzle`)
        (else
          (`self.UpdatePuzzleUI`)
          (`self.CheckForPuzzleCompletion`))))))

(event `/Game/Blueprints/Interfaces/BPI_Puzzle.TogglePuzzleUI`
  (bind _returnvalue (`GameplayStatics.GetPlayerController` 0))
  (bind _bp_cursormanager (`self.BP_CursorManager`))
  (bind _playerui (`/Game/Blueprints/Player/BP_PlayerMain.PlayerUI` (`self.Player`)))
  (set `self.InPuzzle` (not (`self.InPuzzle`)))
  (`/Game/Blueprints/Player/BP_PlayerMain.Swap Camera` (`self.Player`) (`self.PuzzleCamera`))
  (if (`self.InPuzzle`)
    (`/Game/Blueprints/Reusable/BP_CursorManager.EnableCursorAndMovement` _bp_cursormanager true)
    (`self.EnableInput` _returnvalue)
    (`Widget.SetVisibility` _playerui "Hidden")
    (else
      (`/Game/Blueprints/Reusable/BP_CursorManager.EnableCursorAndMovement` _bp_cursormanager false)
      (`self.DisableInput` _returnvalue)
      (`Widget.SetVisibility` _playerui "Visible"))))

(event `/Game/Blueprints/Interfaces/BPI_Interactable.Interact`
  (if (and (not (`self.Solved`)) (not (`self.InPuzzle`)))
    (`self.TogglePuzzleUI`)
    (`/Game/Blueprints/Environment/Interactables/Puzzles/FloorThree/Photoboard/BPW_BP_PhotoboardPuzzleWidgetActor.ToggleUI` (`self.PuzzleUI`) (`self.InPuzzle`))))

(event `/Game/Blueprints/Interfaces/BPI_Puzzle.UpdatePuzzleUI`)

(event `/Game/Blueprints/Interfaces/BPI_Puzzle.CheckForPuzzleCompletion`
  (`self.CheckPuzzleCompletion`))

(event `/Game/Blueprints/Interfaces/BPI_Objective.CompleteObjective`)

(fn `AssignRandomMaterials`)

(fn `CheckPuzzleCompletion`
  (locals (`isPuzzleComplete?` :type Boolean :default true))
  (for _index (range (+ (`KismetArrayLibrary.Array_Length` (`self.PuzzleSlotArray`)) 1))
    (bind _returnvalue (`Image.GetDynamicMaterial` (`|GetArrayItem` (`self.PuzzleImageArray`) _index)))
    (if (not (!= (`PrimitiveComponent.GetMaterial` (`/Game/Blueprints/Environment/Interactables/Puzzles/FloorThree/Photoboard/BP_PhotoboardPuzzleSlot.Plane` (`|GetArrayItem` (`self.PuzzleSlotArray`) _index)) 0) _returnvalue))
      (set `local.isPuzzleComplete?` false)
      (break)
      (elif (`self.InPuzzle`)
        (`KismetSystemLibrary.PrintString` "Puzzle Complete")
        (`self.OnPuzzleCompletion`)
        (elif (== (`self.MovesMade`) (`self.MaxMoves`))
          (`self.TogglePuzzleUI`)
          (`self.ResetPuzzle`))))))

(fn `InitPuzzleSlots`
  (bind _puzzleui (`self.PuzzleUI`))
  (for (_array_element _array_index) (`|MakeArray` (`ChildActorComponent.ChildActor` (`self.BP_PhotoboardPuzzleSlot01`)) (`ChildActorComponent.ChildActor` (`self.BP_PhotoboardPuzzleSlot02`)) (`ChildActorComponent.ChildActor` (`self.BP_PhotoboardPuzzleSlot03`)) (`ChildActorComponent.ChildActor` (`self.BP_PhotoboardPuzzleSlot04`)) (`ChildActorComponent.ChildActor` (`self.BP_PhotoboardPuzzleSlot05`)) (`ChildActorComponent.ChildActor` (`self.BP_PhotoboardPuzzleSlot06`)) (`ChildActorComponent.ChildActor` (`self.BP_PhotoboardPuzzleSlot07`)))
    (bind _asbp_photoboard_puzzle_slot (cast `/Game/Blueprints/Environment/Interactables/Puzzles/FloorThree/Photoboard/BP_PhotoboardPuzzleSlot` _array_element))
    (`KismetArrayLibrary.Array_Set` (`self.PuzzleSlotArray`) _array_index _asbp_photoboard_puzzle_slot)
    (set `/Game/Blueprints/Environment/Interactables/Puzzles/FloorThree/Photoboard/BP_PhotoboardPuzzleSlot.Puzzle` self _asbp_photoboard_puzzle_slot)
    (set `self.PuzzleImageArray` (`|MakeArray` (`/Game/Blueprints/Environment/Interactables/Puzzles/FloorThree/Photoboard/BPW_BP_PhotoboardPuzzleWidgetActor.PuzzlePolaroid01` _puzzleui) (`/Game/Blueprints/Environment/Interactables/Puzzles/FloorThree/Photoboard/BPW_BP_PhotoboardPuzzleWidgetActor.PuzzlePolaroid02` _puzzleui) (`/Game/Blueprints/Environment/Interactables/Puzzles/FloorThree/Photoboard/BPW_BP_PhotoboardPuzzleWidgetActor.PuzzlePolaroid03` _puzzleui) (`/Game/Blueprints/Environment/Interactables/Puzzles/FloorThree/Photoboard/BPW_BP_PhotoboardPuzzleWidgetActor.PuzzlePolaroid04` _puzzleui) (`/Game/Blueprints/Environment/Interactables/Puzzles/FloorThree/Photoboard/BPW_BP_PhotoboardPuzzleWidgetActor.PuzzlePolaroid05` _puzzleui) (`/Game/Blueprints/Environment/Interactables/Puzzles/FloorThree/Photoboard/BPW_BP_PhotoboardPuzzleWidgetActor.PuzzlePolaroid06` _puzzleui) (`/Game/Blueprints/Environment/Interactables/Puzzles/FloorThree/Photoboard/BPW_BP_PhotoboardPuzzleWidgetActor.PuzzlePolaroid07` _puzzleui)))))

(fn `OnPuzzlePieceClicked`
  (params (Button :type "Button Object Reference"))
  (locals (PuzzleSlot :type "/Game/Blueprints/Environment/Interactables/Puzzles/FloorThree/Photoboard/BP_PhotoboardPuzzleSlot Object Reference"))
  (if (`self.Solved`)
    (return)
    (else
      (`self.OnMoveMade`))))

(fn `PuzzleLineTrace`
  (params (PuzzlePiece :type "/Game/Blueprints/Environment/Interactables/Puzzles/FloorThree/Photoboard/BP_PhotoboardPuzzleSlot Object Reference"))
  (bind (_worldlocation _worlddirection) (`PlayerController.DeprojectMousePositionToWorld` (`GameplayStatics.GetPlayerController` 0)))
  (if (not (`self.Solved`))
    (bind _outhit (`KismetSystemLibrary.LineTraceSingle` _worldlocation (+ _worldlocation (* _worlddirection 150.0)) "TraceTypeQuery1"))
    (bind (_bblockinghit _binitialoverlap _time _distance _location _impactpoint _normal _impactnormal _physmat _hitactor) (`GameplayStatics.BreakHitResult` _outhit))
    (if (`KismetStringLibrary.Contains` (`KismetSystemLibrary.GetDisplayName` _hitactor) "Slot")
      (bind _asbp_photoboard_puzzle_slot (cast `/Game/Blueprints/Environment/Interactables/Puzzles/FloorThree/Photoboard/BP_PhotoboardPuzzleSlot` _hitactor))
      (set `self.CurrentHoveredPuzzlePiece` _asbp_photoboard_puzzle_slot)
      (set `self.CanClick` true)
      (else
        (set `self.CanClick` false)
        (return)))
    (else
      (return))))

(fn `SetMaterial`
  (params (PuzzleSlot :type "/Game/Blueprints/Environment/Interactables/Puzzles/FloorThree/Photoboard/BP_PhotoboardPuzzleSlot Object Reference") (NewMaterial :type "MaterialInstance Object Reference"))
  (`PrimitiveComponent.SetMaterial` (`/Game/Blueprints/Environment/Interactables/Puzzles/FloorThree/Photoboard/BP_PhotoboardPuzzleSlot.Plane` PuzzleSlot) 0 NewMaterial))

(fn `UserConstructionScript`
  (`parent.UserConstructionScript`))