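; Interactable sliding-image puzzle actor that lets the player enter a puzzle view and records its completion.
; Interact calls TogglePuzzleUI only when not already in the puzzle; the toggle passes the puzzle camera to the player's SwapCamera and flips cursor, movement and actor input.
; CompletePuzzle reports the puzzle name to the game instance under the hardcoded FLOORTWO level and saves completion.
; The tile-sliding logic is not in these graphs.
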(event `/Game/Blueprints/Environment/Interactables/Puzzles/BPI_Puzzle.TogglePuzzleUI`
  (bind _returnvalue (`GameplayStatics.GetPlayerController` 0))
  (bind _bp_cursormanager (`self.BP_CursorManager`))
  (set `self.InPuzzle` (not (`self.InPuzzle`)))
  (bind _asbp_player_main (cast `/Game/Blueprints/Player/BP_PlayerMain` (`GameplayStatics.GetPlayerCharacter` 0)))
  (`/Game/Blueprints/Player/BP_PlayerMain.Swap Camera` _asbp_player_main (`self.PuzzleCamera`))
  (if (`self.InPuzzle`)
    (`/Game/Blueprints/Reusable/BP_CursorManager.EnableCursorAndMovement` _bp_cursormanager false)
    (`self.DisableInput` _returnvalue)
    (else
      (`/Game/Blueprints/Reusable/BP_CursorManager.EnableCursorAndMovement` _bp_cursormanager true)
      (`self.EnableInput` _returnvalue))))

(event `/Game/Blueprints/Environment/Interactables/Puzzles/BPI_Puzzle.CompletePuzzle`
  (bind _outgameinstance (`/Game/Blueprints/Reusable/BP_RefToGameInstance.GetRefToGameInstance` (`self.BP_RefToGameInstance`)))
  (`/Game/Blueprints/Data/BP_GameInstanceClass.Complete Puzzle in Scene` _outgameinstance "FLOORTWO" (`self.PuzzleName`))
  (`/Game/Blueprints/Data/BP_GameInstanceClass.SavePuzzleCompletion` _outgameinstance self))

(event `/Game/Blueprints/Environment/Interactables/BPI_Interactable.Interact`
  (if (not (`self.InPuzzle`))
    (`self.TogglePuzzleUI`)))

(fn `UserConstructionScript`
  (`parent.UserConstructionScript`))