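; BP_LobbyCeilingLight is a lobby ceiling light actor that can be toggled on and off.
; Its ToggleLight event sets the light component's visibility from Active, swaps the mesh's first material between on and off variants to match, then inverts Active.
; It has no active BeginPlay, overlap or Tick logic, and the construction script only calls its parent.
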(event `self.ToggleLight`
  (params (Active :type Boolean))
  (`SceneComponent.SetVisibility` (`self.Light`) Active false)
  (`PrimitiveComponent.SetMaterial` (`self.LightMesh`) 0 (select `bool` (`self.Active`) :`false` (`self.LightOffMaterial`) :`true` (`self.LightOnMaterial`) :!type "MaterialInterface Object Reference"))
  (set `self.Active` (not (`self.Active`))))

(fn `UserConstructionScript`
  (`parent.UserConstructionScript`))