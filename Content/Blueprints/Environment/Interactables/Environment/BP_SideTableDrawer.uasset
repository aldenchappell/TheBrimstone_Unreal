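; BP_SideTableDrawer is an interactable side table drawer that slides open and closed.
; Interact calls ToggleDrawer, which, when IsInteractable is true, plays DrawerTimeline or reverses it from the end based on IsOpen.
; Timeline updates set the Drawer's relative location through VInterpTo, using the float track as DeltaTime toward a fixed offset.
; IsOpen flips on every timeline update rather than once on completion.
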(event `ToggleDrawer`
  (if (`self.IsInteractable`)
    (if (`self.IsOpen`)
      (bind (_direction _drawerfloattrack) (`Timeline|DrawerTimeline` :!via `ReverseFromEnd` :!label _label)
        (:`Update`
          (`SceneComponent.K2_SetRelativeLocation` (`self.Drawer`) (`KismetMathLibrary.VInterpTo` (0.0 0.0 0.0) (0.0 20.0 0.0) _drawerfloattrack 5.0) false false)
          (set `self.IsOpen` (not (`self.IsOpen`)))))
      (else
        (goto _label)))))

(event `/Game/Blueprints/Interfaces/BPI_Interactable.Interact`
  (`self.ToggleDrawer`))

(fn `UserConstructionScript`
  (`parent.UserConstructionScript`))