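; BP_ElevatorButton is an interactable button actor that holds a reference to a BP_Elevator.
; On BeginPlay, if the Elevator reference is not set, it takes the first BP_Elevator found in the level.
; Its Interact event is empty, so it does not yet operate the elevator, and the construction script only calls the parent.
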(event `self.ReceiveBeginPlay`
  (`parent.ReceiveBeginPlay`)
  (`/Engine/EditorBlueprintResources/StandardMacros.IsValid` (`self.Elevator`)
    (:`Is Not Valid`
      ;[1 1 1] if null, get reference to elevator
      (bind _outactors (`GameplayStatics.GetAllActorsOfClass` "/Game/Blueprints/Environment/BP_Elevator.BP_Elevator_C"))
      (set `self.Elevator` (`|GetArrayItem` _outactors)))))

(event `/Game/Blueprints/Environment/Interactables/BPI_Interactable.Interact`)

(fn `UserConstructionScript`
  (`parent.UserConstructionScript`))