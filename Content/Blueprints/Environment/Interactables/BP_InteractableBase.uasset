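; Base Blueprint for interactable world objects that can act as inventory pickups or be placed from the player's inventory.
; Interact runs only when the lobby is completed and the object is interactable, or lobby state is ignored, then adds pickups to BP_PlayerMain's inventory component.
; OnPlaceObject removes the placed item from that inventory, with both paths refreshing the inventory UI.
; PickupItem triggers Interact and returns the object itself; the destroy logic is unconnected.
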(event `/Game/Blueprints/Interfaces/BPI_Interactable.Interact`
  (bind _outgameinstance (`/Game/Blueprints/Reusable/BP_RefToGameInstance.GetRefToGameInstance` (`self.BP_RefToGameInstance`)))
  (if (or (and (`/Game/Blueprints/Data/BP_GameInstanceClass.IsLobbyCompleted` _outgameinstance) (`self.IsInteractable`)) (`self.IgnoreLobbyState`))
    (`self.Interact`)
    (bind _asbp_player_main (cast `/Game/Blueprints/Player/BP_PlayerMain` (`GameplayStatics.GetPlayerCharacter` 0)))
    (if (`self.IsPickup`)
      (bind _bp_playerinventory (`/Game/Blueprints/Player/BP_PlayerMain.BP_PlayerInventory` _asbp_player_main))
      (`/Game/Blueprints/Player/Inventory/BP_PlayerInventory.AddItemToInventory` _bp_playerinventory self)
      (`/Game/Blueprints/Player/Inventory/BP_PlayerInventory.UpdateInventoryUI` _bp_playerinventory))))

(event `Destroy`)

(event `OnPlaceObject`
  (params (ItemToPlace :type "/Game/Blueprints/Environment/Interactables/BP_InteractableBase Object Reference (by ref)"))
  (bind _asbp_player_main (cast `/Game/Blueprints/Player/BP_PlayerMain` (`GameplayStatics.GetPlayerCharacter` 0)))
  (bind _bp_playerinventory (`/Game/Blueprints/Player/BP_PlayerMain.BP_PlayerInventory` _asbp_player_main))
  (`/Game/Blueprints/Player/Inventory/BP_PlayerInventory.RemoveItemFromInventory` _bp_playerinventory ItemToPlace)
  (`/Game/Blueprints/Player/Inventory/BP_PlayerInventory.UpdateInventoryUI` _bp_playerinventory))

(fn `PickupItem`
  (returns (Interactable :type "/Game/Blueprints/Environment/Interactables/BP_InteractableBase Object Reference"))
  (`self.Interact`)
  (if (`self.IsPickup`)
    (return self)
    (else
      (return self))))

(fn `UserConstructionScript`)