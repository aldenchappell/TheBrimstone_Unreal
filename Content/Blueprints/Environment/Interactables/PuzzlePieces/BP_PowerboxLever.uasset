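; BP_PowerboxLever is a clickable powerbox lever puzzle piece that completes the lobby puzzle.
; A click while interactable marks the lobby completed on the game instance, updates its lights, saves completion and registers the puzzle as done in LOBBY.
; A timeline then rolls the mesh, with each update also requesting the switch sound from BP_EnvironmentalSoundPlayer and, if that actor exists, disabling interaction.
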(event `/Game/Blueprints/Interfaces/BPI_Clickable.OnClickedEvent`
  (if (`self.IsInteractable`)
    (`self.Interact`)
    (bind (_direction _levertrackfloat) (`Timeline|LeverTimeline`)
      (:`Update`
        (`SceneComponent.K2_SetRelativeRotation` (`self.Mesh`) (`KismetMathLibrary.MakeRotator` (`KismetMathLibrary.Lerp` 0.0 90.0 _levertrackfloat)) false false)
        (bind _returnvalue (`GameplayStatics.GetActorOfClass` "/Game/Blueprints/Environment/BP_EnvironmentalSoundPlayer.BP_EnvironmentalSoundPlayer_C"))
        (`/Engine/EditorBlueprintResources/StandardMacros.IsValid` _returnvalue
          (:`Is Valid`
            (`/Game/Blueprints/Environment/BP_EnvironmentalSoundPlayer.PlaySound2D` _returnvalue "/Game/Sound/GeneralSFX/Big_switch_sound_effect_1.Big_switch_sound_effect_1")
            (set `self.IsInteractable` false)))))))

(event `/Game/Blueprints/Interfaces/BPI_Interactable.Interact`
  (`self.CompletePuzzle`))

(event `/Game/Blueprints/Environment/Interactables/Puzzles/BPI_Puzzle.CompletePuzzle`
  (bind _outgameinstance (`/Game/Blueprints/Reusable/BP_RefToGameInstance.GetRefToGameInstance` (`self.BP_RefToGameInstance`)))
  (set `/Game/Blueprints/Data/BP_GameInstanceClass.IsLobbyCompleted` true _outgameinstance)
  (`/Game/Blueprints/Data/BP_GameInstanceClass.HandleLobbyLights` _outgameinstance)
  (`/Game/Blueprints/Data/BP_GameInstanceClass.SavePuzzleCompletion` _outgameinstance self)
  (`/Game/Blueprints/Data/BP_GameInstanceClass.Complete Puzzle in Scene` _outgameinstance "LOBBY" (`self.PuzzleName`)))

(event `/Game/Blueprints/Environment/Interactables/Puzzles/BPI_Puzzle.TogglePuzzleUI`)

(fn `UserConstructionScript`
  (`parent.UserConstructionScript`))