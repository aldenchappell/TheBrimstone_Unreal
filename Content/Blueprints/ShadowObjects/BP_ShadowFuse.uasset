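; BP_ShadowFuse is a clickable shadow object that lets the player place an inventory fuse into the powerbox.
; When clicked while interactable, it searches the player's inventory slots for an item named "Fuse", printing other items' names.
; A match is passed to BP_Powerbox, found by class, then removed from the inventory before the shadow destroys itself and the inventory UI refreshes.
; The loop's exit also feeds the name check.
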(event `/Game/Blueprints/Interfaces/BPI_Clickable.OnClickedEvent`
  (if (`self.IsInteractable`)
    (bind _asbp_player_main (cast `/Game/Blueprints/Player/BP_PlayerMain` (`GameplayStatics.GetPlayerCharacter` 0)))
    (bind _bp_playerinventory (`/Game/Blueprints/Player/BP_PlayerMain.BP_PlayerInventory` _asbp_player_main))
    (bind _newinventoryslots (`/Game/Blueprints/Player/Inventory/BP_PlayerInventory.NewInventorySlots` _bp_playerinventory))
    (for (_ _array_index) _newinventoryslots
      (bind _item (break `/Game/Blueprints/Structs/STR_InventorySlot` (`|GetArrayItem` _newinventoryslots _array_index)))
      (if (`KismetSystemLibrary.IsValid` _item)
        (if (== (`/Game/Blueprints/Environment/Interactables/BP_InteractableBase.InteractableName` _item) "Fuse") :!label _label
          (bind _returnvalue (`GameplayStatics.GetActorOfClass` "/Game/Blueprints/Environment/Interactables/Puzzles/Lobby/FuseBox/BP_Powerbox.BP_Powerbox_C"))
          (`/Game/Blueprints/Environment/Interactables/BP_InteractableBase.OnPlaceObject` _returnvalue _item)
          (`/Game/Blueprints/Player/Inventory/BP_PlayerInventory.RemoveItemFromInventory` _bp_playerinventory _item)
          (`self.K2_DestroyActor`)
          (`/Game/Blueprints/Player/Inventory/BP_PlayerInventory.UpdateInventoryUI` _bp_playerinventory)
          (else
            (`KismetSystemLibrary.PrintString` (`KismetSystemLibrary.GetDisplayName` _item))))))
    (goto _label)))

(fn `UserConstructionScript`
  (`parent.UserConstructionScript`))