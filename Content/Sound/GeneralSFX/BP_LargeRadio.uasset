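; BP_LargeRadio is an interactable radio actor that switches its audio on and off.
; Interact calls ToggleRadio only when the game instance reports the lobby is completed, while SetPlay calls it unconditionally.
; ToggleRadio flips the Playing flag and adjusts the volume multiplier.
; Tick enforces that flag every frame, calling Play from the start while it is set and Stop otherwise.
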(event `self.ReceiveTick`
  (params (DeltaSeconds :type "Float (single-precision)"))
  (`parent.ReceiveTick` DeltaSeconds)
  (if (`self.Playing`)
    (`AudioComponent.Play` (`self.Audio`) 0.0)
    (else
      (`AudioComponent.Stop` (`self.Audio`)))))

(event `/Game/Blueprints/Environment/Interactables/BPI_Interactable.Interact`
  (bind _outgameinstance (`/Game/Blueprints/Reusable/BP_RefToGameInstance.GetRefToGameInstance` (`self.BP_RefToGameInstance`)))
  (if (`/Game/Blueprints/Data/BP_GameInstanceClass.IsLobbyCompleted` _outgameinstance)
    (`self.ToggleRadio`)))

(fn `SetPlay`
  (`self.ToggleRadio`)
  (return))

(fn `ToggleRadio`
  (bind _audio (`self.Audio`))
  (if (not (`self.Playing`))
    (`AudioComponent.SetVolumeMultiplier` _audio 0.41)
    (else
      (`AudioComponent.SetVolumeMultiplier` _audio 1.0)))
  (set `self.Playing` (not (`self.Playing`)))
  (return))

(fn `UserConstructionScript`
  (`parent.UserConstructionScript`))